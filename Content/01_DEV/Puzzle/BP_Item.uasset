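; BP_Item is an interactable puzzle item that the player either picks up or combines with a held inventory item, depending on its Typ.
; Pickups pass their name, mesh, materials, transform and class to the player's inventory, send a valid message to linked actors, then destroy themselves.
; Crafting items require the selected item to match NeedToCraft, then consume it and replace themselves with CurdSoapRub, otherwise showing a German monologue hint.
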(event `/Game/01_DEV/Interface_and_Self/Interface_Interactable.Interact`
  (params (Player_ID :type "/Game/01_DEV/BP_Player Object Reference"))
  (bind _mesh (`self.Mesh`))
  (bind _inventory (`/Game/01_DEV/BP_Player.Inventory` Player_ID))
  (bind _currentintemindex (`/Game/01_DEV/BP_Player.CurrentIntemIndex` Player_ID))
  (bind _staticmesh (`StaticMeshComponent.StaticMesh` _mesh))
  (if (== (`self.Typ`) 1)
    (`/Game/01_DEV/BP_Player.CurrentInventory` Player_ID (make `/Game/01_DEV/Puzzle/ItemStructure` (`KismetSystemLibrary.GetDisplayName` _staticmesh) _staticmesh (`MeshComponent.GetMaterials` _mesh) (`KismetMathLibrary.MakeTransform` (`SceneComponent.RelativeLocation` _mesh) (`SceneComponent.RelativeRotation` _mesh) (`SceneComponent.K2_GetComponentScale` _mesh)) (`GameplayStatics.GetObjectClass` self)))
    (for _array_element (`self.ActortoReact`)
      (message `/Game/01_DEV/Interface_and_Self/Interface_Interactable.SetValid` _array_element true))
    (`self.K2_DestroyActor`)
    (elif (== (`self.Typ`) 4)
      (if (`KismetStringLibrary.EqualEqual_StrStr` (`.Name_5_1C06FF694E268D40E70FD589ADD5300D` (break `/Game/01_DEV/Puzzle/ItemStructure` (`|GetArrayItem` _inventory _currentintemindex))) (`self.NeedToCraft`))
        (`|SpawnActorFromClass` "/Game/01_DEV/Puzzle/03_Craft/CurdSoapRub.CurdSoapRub_C" (`SceneComponent.K2_GetComponentToWorld` (`self.Mesh`)) "Undefined" "MultiplyWithRoot" null null)
        (`KismetArrayLibrary.Array_Remove` _inventory _currentintemindex)
        (`/Game/01_DEV/BP_Player.ShowItem` Player_ID)
        (`self.K2_DestroyActor`)
        (else
          (`/Game/01_DEV/Interface_and_Self/FL_Utils.SetNewSelfMonolog` (`GameplayStatics.GetPlayerController` 0) "Forward" "Ich brauche etwas anderes"))))))

(event `/Game/01_DEV/Interface_and_Self/Interface_Interactable.SetValid`
  (params (SetValid :type Boolean))
  (set `self.IsValid` SetValid))

(fn `Solved`
  (returns (SetSolved :type Boolean))
  (return false))

(fn `UserConstructionScript`)

(fn `Valid`
  (returns (Interactable :type Boolean) (Typ :type "/Game/01_DEV/Puzzle/E_Interactable_Type Enum"))
  (return (`self.IsValid`) (`self.Typ`)))