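; BP_SecretDoor is an interactable secret door in the wardrobe puzzle that slides open when used.
; Its validity flag is set externally through SetValid and reported as interactability by Valid, while Solved always returns false.
; Interact moves the door component sideways, clears the flag and shows a German HUD monologue hinting that the broken camera needs a wrench.
; It then sends a valid message to ActorToReact, enabling the next puzzle step.
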(event `/Game/01_DEV/Interface_and_Self/Interface_Interactable.SetValid`
  (params (SetValid :type Boolean))
  (set `self.Set Valid` SetValid))

(event `/Game/01_DEV/Interface_and_Self/Interface_Interactable.Interact`
  (params (Player_ID :type "/Game/01_DEV/BP_Player Object Reference"))
  (`KismetSystemLibrary.MoveComponentTo` (`self.SecretDoor_SeecretDoor`) (0.0 80.0 0.0))
  (set `self.Set Valid` false)
  (bind _hud (message `/Game/01_DEV/Interface_and_Self/IF_HUD.Call to HUD` (`PlayerController.GetHUD` (`GameplayStatics.GetPlayerController` 0))))
  (`/Game/03_UI/AWB_PlayerHUD.ShowMonolog` (`/Game/01_DEV/HUD_PMP.PlayerHUD` _hud) "Ach verdammt, die Kamera ist kaputt. \nIch sollte etwas zum reapieren finden. Vielleicht einen Schrauben schlüssel.")
  (message `/Game/01_DEV/Interface_and_Self/Interface_Interactable.SetValid` (`self.ActorToReact`) true))

(fn `Solved`
  (returns (SetSolved :type Boolean))
  (return false))

(fn `UserConstructionScript`)

(fn `Valid`
  (returns (Interactable :type Boolean) (Typ :type "/Game/01_DEV/Puzzle/E_Interactable_Type Enum"))
  (return (`self.Set Valid`) "NewEnumerator2"))