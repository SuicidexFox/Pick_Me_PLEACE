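; BP_Wardrobe is an interactable wardrobe puzzle pawn that the player temporarily possesses.
; Interact freezes the player, slides the right door, smoothly possesses the wardrobe and pushes a fading widget onto the HUD stack.
; Leave restores player, control rotation and door; if solved, it disables interaction, validates a linked actor, slides the left door and may trigger the game mode's Finale, depending on a saved SolvedSorted flag.
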(event `/Game/01_DEV/Interface_and_Self/Interface_Interactable.Interact`
  (params (Player_ID :type "/Game/01_DEV/BP_Player Object Reference"))
  (`|ExecutionSequence`
    (:`then_0`
      (bind _output_get (set `self.Player ID` Player_ID))
      (set `self.PlayerControlRotation` (`self.GetControlRotation` Player_ID))
      (set `/Game/01_DEV/BP_Player.CanMove` false _output_get)
      (`/Game/01_DEV/Interface_and_Self/ML_Utils.SmothPossess` (`GameplayStatics.GetPlayerController` 0) self
        (:`Compledet`
          (set `self.PossessEnd` true))
        (:`then`
          (bind _returnvalue (`CommonActivatableWidgetContainerBase.BP_AddWidget` (`/Game/01_DEV/Interface_and_Self/FL_Utils.GetOverlayStacks` (`GameplayStatics.GetPlayerController` 0)) "/Game/03_UI/DragAndDrop/AWB_Wardrobe.AWB_Wardrobe_C"))
          (bind _output_get_2 (set `self.CurrentWidget` _returnvalue))
          (`UserWidget.PlayAnimationForward` _output_get_2 (`/Game/03_UI/DragAndDrop/AWB_Wardrobe.Anim_Opacity` _output_get_2) 1.0 false)
          (set `/Game/03_UI/DragAndDrop/AWB_Wardrobe.ParentPawn` self _returnvalue))))
    (:`then_1`
      (`KismetSystemLibrary.MoveComponentTo` (`self.Wardrobe_Door_r`) (0.0 75.0 0.0) (struct) true true 1.0))))

(event `Leave`
  (bind _returnvalue (`GameplayStatics.GetPlayerController` 0))
  (bind _player_id (`self.Player ID`))
  (bind _currentwidget (`self.CurrentWidget`))
  (`/Game/01_DEV/Interface_and_Self/ML_Utils.SmothPossess` _returnvalue _player_id
    (:`Compledet`
      (`Controller.SetControlRotation` _returnvalue (`self.PlayerControlRotation`))
      (set `/Game/01_DEV/BP_Player.CanMove` true _player_id)
      (`CommonActivatableWidgetContainerBase.RemoveWidget` (`/Game/01_DEV/Interface_and_Self/FL_Utils.GetOverlayStacks` (`GameplayStatics.GetPlayerController` 0)) (`self.CurrentWidget`))
      (`UserWidget.PlayAnimationReverse` _currentwidget (`/Game/03_UI/DragAndDrop/AWB_Wardrobe.Anim_Opacity` _currentwidget) 1.0 false)
      (set `self.PossessEnd` false)
      (`KismetSystemLibrary.MoveComponentTo` (`self.Wardrobe_Door_r`) (0.0 0.0 0.0) (struct) true true 1.0)
      (if (`self.isSolved`)
        (set `self.Set Valid` false)
        (message `/Game/01_DEV/Interface_and_Self/Interface_Interactable.SetValid` (`self.ActorToReact`) true)
        (`KismetSystemLibrary.Delay` 0.5)
        (`KismetSystemLibrary.MoveComponentTo` (`self.Wardrobe_Door_l`) (0.0 -80.0 0.0) (struct) true true 1.0)
        (if (`/Game/01_DEV/SaveGame_Gameplay.SolvedSorted` (`/Game/01_DEV/Interface_and_Self/FL_Utils.GetSG_Gameplay` (`GameplayStatics.GetGameInstance`)))
          (`/Game/01_DEV/GameMode_PMP.Finale` (`/Game/01_DEV/Interface_and_Self/FL_Utils.GetGM_PMP` (`GameplayStatics.GetGameMode`))))))))

(event `/Game/01_DEV/Interface_and_Self/Interface_Interactable.SetValid`
  (params (SetValid :type Boolean))
  (set `self.Set Valid` SetValid))

(fn `Solved`
  (returns (SetSolved :type Boolean))
  (return false))

(fn `UserConstructionScript`)

(fn `Valid`
  (returns (Interactable :type Boolean) (Typ :type "/Game/01_DEV/Puzzle/E_Interactable_Type Enum"))
  (return (`self.Set Valid`) "NewEnumerator3"))