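; Washing machine puzzle station that opens its door and becomes interactable once Solved fires.
; Interact checks the held inventory item by name: socks on the first use, then detergent, consuming matches, animating door and drawer, or showing German monologue hints.
; Detergent triggers a smooth possess of the machine with an inspect widget.
; Move input turns the program dial; confirming the correct position lights the body, returns control and disables interaction.
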(event `/Game/01_DEV/Interface_and_Self/Interface_Interactable.Solved`
  (`KismetSystemLibrary.MoveComponentTo` (`self.Washingmachine_Bullauge`) (-25.0 -25.0 43.0) (struct :`Yaw` 100.0) true true 1.0)
  (set `self.IsInteractable` true))

(event `/Game/01_DEV/Interface_and_Self/Interface_Interactable.Interact`
  (params (Player_ID :type "/Game/01_DEV/BP_Player Object Reference"))
  (bind _playerid (`self.PlayerID`))
  (bind _washingmachine_auszug (`self.Washingmachine_Auszug`))
  (bind _playerid_2 (`self.PlayerID`))
  (bind _washingmachine_auszug_2 (`self.Washingmachine_Auszug`))
  (bind _playerid_3 (`self.PlayerID`))
  (bind _inventory (`/Game/01_DEV/BP_Player.Inventory` _playerid_2))
  (bind _currentintemindex (`/Game/01_DEV/BP_Player.CurrentIntemIndex` _playerid_2))
  (bind _name (break `/Game/01_DEV/Puzzle/ItemStructure` (`|GetArrayItem` _inventory _currentintemindex)))
  (bind _output_get (set `self.PlayerID` Player_ID))
  (if (`self.IsInteractable`)
    (`/Engine/EditorBlueprintResources/StandardMacros.DoOnceWithAfter`
      (:`Once`
        ;[1 1 1] Socks
        (if (`KismetStringLibrary.EqualEqual_StrStr` (`.Name_5_1C06FF694E268D40E70FD589ADD5300D` (break `/Game/01_DEV/Puzzle/ItemStructure` (`|GetArrayItem` (`/Game/01_DEV/BP_Player.Inventory` _output_get) (`/Game/01_DEV/BP_Player.CurrentIntemIndex` _output_get)))) (`|GetArrayItem` (`self.NeedDetergent`)))
          (`KismetSystemLibrary.MoveComponentTo` (`self.Washingmachine_Bullauge`) (-25.0 -25.0 43.0) (struct) true true 1.0)
          (`KismetArrayLibrary.Array_Remove` (`/Game/01_DEV/BP_Player.Inventory` _playerid) (`/Game/01_DEV/BP_Player.CurrentIntemIndex` _playerid))
          (`/Game/01_DEV/BP_Player.ShowItem` _playerid)
          (`KismetSystemLibrary.MoveComponentTo` _washingmachine_auszug (- (`SceneComponent.RelativeLocation` _washingmachine_auszug) (-11.0 0.0 0.0)) (`SceneComponent.RelativeRotation` _washingmachine_auszug) true true 1.0)))
      (:`After`
        ;[1 1 1] Detergent
        (if (`KismetStringLibrary.EqualEqual_StrStr` (`|GetArrayItem` (`self.NeedDetergent`) 1) _name)
          (`KismetArrayLibrary.Array_Remove` _inventory _currentintemindex)
          (`/Game/01_DEV/BP_Player.ShowItem` _playerid_3)
          (`KismetSystemLibrary.MoveComponentTo` _washingmachine_auszug_2 (+ (`SceneComponent.RelativeLocation` _washingmachine_auszug_2) (11.0 0.0 0.0)) (`SceneComponent.RelativeRotation` _washingmachine_auszug_2) true true 1.0)
          (`self.SetupPossess`)
          (elif (`KismetStringLibrary.EqualEqual_StrStr` (`|GetArrayItem` (`self.NeedDetergent`) 2) _name)
            (`KismetArrayLibrary.Array_Remove` (`/Game/01_DEV/BP_Player.Inventory` _playerid_3) (`/Game/01_DEV/BP_Player.CurrentIntemIndex` _playerid_3))
            (`/Game/01_DEV/BP_Player.ShowItem` _playerid_3)
            (`/Game/01_DEV/Interface_and_Self/FL_Utils.SetNewSelfMonolog` (`GameplayStatics.GetPlayerController` 0) "Forward" "dass ist leer..... verdammt.  \nich muss wohl was anderes finden")
            (else
              (`/Engine/EditorBlueprintResources/StandardMacros.DoOnce` false
                (:`Completed`
                  (`/Game/01_DEV/Interface_and_Self/FL_Utils.SetNewSelfMonolog` (`GameplayStatics.GetPlayerController` 0) "Forward" "ich muss waschmittel finden"))))))))))

(event `SetupPossess`
  (bind _playerid (`self.PlayerID`))
  ;[1 1 1] Wash Programm
  (set `self.PlayerControllerRotation` (`self.GetControlRotation` _playerid))
  (set `/Game/01_DEV/BP_Player.CanMove` false _playerid)
  (`|ExecutionSequence`
    (:`then_0`
      (`/Game/01_DEV/Interface_and_Self/ML_Utils.SmothPossess` (`GameplayStatics.GetPlayerController` 0) self
        (:`Compledet`
          (set `self.PossessEnd` true))
        (:`then`
          (`MeshComponent.SetOverlayMaterial` (`self.Washingmachine_Button`) "/Game/04_Material/M_Shader.M_Shader")
          ;[1 1 1] Widget
          (bind _returnvalue (`CommonActivatableWidgetContainerBase.BP_AddWidget` (`/Game/01_DEV/Interface_and_Self/FL_Utils.GetOverlay` (`GameplayStatics.GetPlayerController` 0)) "/Game/02_UI/AWB_Inspacted.AWB_Inspacted_C"))
          (bind _output_get (set `self.CurrentWidget` _returnvalue))
          (`UserWidget.PlayAnimationForward` _output_get (`/Game/02_UI/AWB_Inspacted.Anim_Opacity` _output_get) 1.0 false))))))

(event `EnhancedInput|/Game/01_DEV/Input/IA_Tab`
  (params (ActionValue :type Boolean) (ElapsedSeconds :type "Float (double-precision)") (TriggeredSeconds :type "Float (double-precision)") (InputAction :type "InputAction Object Reference" :default "/Game/01_DEV/Input/IA_Tab.IA_Tab"))
  (bind _returnvalue (`GameplayStatics.GetPlayerController` 0))
  (bind _currentwidget (`self.CurrentWidget`))
  (bind _playerid (`self.PlayerID`))
  ;[1 1 1] Laeve
  (:`Started`
    (`/Game/01_DEV/Interface_and_Self/ML_Utils.SmothPossess` _returnvalue _playerid :!label _label
      (:`Compledet`
        (`Controller.SetControlRotation` _returnvalue (`self.PlayerControllerRotation`))
        (set `/Game/01_DEV/BP_Player.CanMove` true _playerid)
        (`CommonActivatableWidgetContainerBase.RemoveWidget` (`/Game/01_DEV/Interface_and_Self/FL_Utils.GetOverlay` (`GameplayStatics.GetPlayerController` 0)) (`self.CurrentWidget`)))
      (:`then`
        (`UserWidget.PlayAnimationReverse` _currentwidget (`/Game/02_UI/AWB_Inspacted.Anim_Opacity` _currentwidget) 1.0 false)
        (set `self.PossessEnd` false)))))

(event `Leave`
  ;[1 1 1] Laeve
  (goto _label))

(event `EnhancedInput|/Game/01_DEV/Input/IA_Interact`
  (params (ActionValue :type Boolean) (ElapsedSeconds :type "Float (double-precision)") (TriggeredSeconds :type "Float (double-precision)") (InputAction :type "InputAction Object Reference" :default "/Game/01_DEV/Input/IA_Interact.IA_Interact"))
  ;[1 0.7602 0.1816] Submit
  (:`Started`
    (if (and (`self.PossessEnd`) (== (`self.CurrentPosition`) 2))
      (`SceneComponent.K2_SetRelativeLocation` (`self.Washingmachine_Button`) (-24.0 0.0 79.0) true false)
      (`MeshComponent.SetScalarParameterValueOnMaterials` (`self.Washingmachine_Korpus`) "Emissive" 1.0)
      (`self.Leave`)
      (set `self.IsInteractable` false)
      (else
        (`KismetSystemLibrary.PrintText` "Sound für falsches Eingabe" true true (struct :`G` 0.66 :`B` 1.0 :`A` 1.0) 2.0 "Waschmaschine")))))

(event `EnhancedInput|/Game/01_DEV/Input/IA_Move`
  (params (ActionValue :type "Vector2D Structure") (ElapsedSeconds :type "Float (double-precision)") (TriggeredSeconds :type "Float (double-precision)") (InputAction :type "InputAction Object Reference" :default "/Game/01_DEV/Input/IA_Move.IA_Move"))
  (bind _currentposition (`self.CurrentPosition`))
  (bind _currentposition_2 (`self.CurrentPosition`))
  ;[1 0.7602 0.1816] Up/Down
  (:`Started`
    (if (and (`self.PossessEnd`) (< ActionValue_Y 0.0))
      (if (not (== 3 _currentposition_2))
        (bind _result (`/Engine/EditorBlueprintResources/StandardMacros.IncrementInt` _currentposition_2)
          (:`  `
            (`SceneComponent.K2_SetRelativeRotation` (`self.Washingmachine_Button`) (`|GetArrayItem` (`self.RotationPosition`) _result) true false))))
      (elif (not (== 0 _currentposition))
        (bind _result_2 (`/Engine/EditorBlueprintResources/StandardMacros.DecrementInt` _currentposition)
          (:`  `
            (`SceneComponent.K2_SetRelativeRotation` (`self.Washingmachine_Button`) (`|GetArrayItem` (`self.RotationPosition`) _result_2) true false)))))))

(fn `SetSolved`
  (returns (SetSolved :type Boolean))
  (return false))

(fn `UserConstructionScript`)

(fn `Valid`
  (returns (Interactable :type Boolean) (Typ :type "/Game/01_DEV/Puzzle/E_Interactable_Type Enum"))
  (return (`self.IsInteractable`) (`self.Typ`)))