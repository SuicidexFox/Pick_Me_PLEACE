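; BP_ItemSocket is an interactable puzzle socket that takes the player's selected inventory item.
; Interact spawns that item at the socket before comparing its name with NeedItem.
; A match disables the socket, sends solved messages to ActorsToReact and removes the inventory entry; a mismatch only shows a German HUD monologue, leaving the spawned actor.
; Valid allows interaction only while enabled and empty, SetValid forwards to the placed item, and Solved always returns false.
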(event `/Game/01_DEV/Interface_and_Self/Interface_Interactable.Interact`
  (params (Player_ID :type "/Game/01_DEV/BP_Player Object Reference"))
  (bind _inventory (`/Game/01_DEV/BP_Player.Inventory` Player_ID))
  (bind _currentintemindex (`/Game/01_DEV/BP_Player.CurrentIntemIndex` Player_ID))
  (bind (_name _mesh _materials _transform _class) (break `/Game/01_DEV/Puzzle/ItemStructure` (`|GetArrayItem` _inventory _currentintemindex)))
  (if (`KismetStringLibrary.NotEqual_StrStr` _name)
    (`self.CurrentItem`
      (:`then`)
      (:`else`
        (bind _returnvalue (`|SpawnActorFromClass` _class (`SceneComponent.K2_GetComponentToWorld` (`self.Scene`)) "Undefined" "MultiplyWithRoot" null null))
        (bind _output_get (set `self.CurrentItem` _returnvalue))
        (if (`KismetStringLibrary.EqualEqual_StrStr` (`self.NeedItem`) _name)
          (message `/Game/01_DEV/Interface_and_Self/Interface_Interactable.SetTyp` _output_get "NewEnumerator3")
          (set `self.Set Valid` false)
          (for _array_element (`self.ActorsToReact`)
            (message `/Game/01_DEV/Interface_and_Self/Interface_Interactable.Set Solved` _array_element))
          (`KismetArrayLibrary.Array_Remove` _inventory _currentintemindex)
          (`/Game/01_DEV/BP_Player.ShowItem` Player_ID)
          (else
            (bind _hud (message `/Game/01_DEV/Interface_and_Self/IF_HUD.Call to HUD` (`PlayerController.GetHUD` (`GameplayStatics.GetPlayerController` 0))))
            (`/Game/03_UI/AWB_PlayerHUD.ShowMonolog` (`/Game/01_DEV/HUD_PMP.PlayerHUD` _hud) "Ich brauche etwas anders")))))))

(event `/Game/01_DEV/Interface_and_Self/Interface_Interactable.SetValid`
  (params (SetValid :type Boolean))
  (bind _output_get (set `self.Set Valid` SetValid))
  (message `/Game/01_DEV/Interface_and_Self/Interface_Interactable.SetValid` (`self.CurrentItem`) _output_get))

(fn `Solved`
  (returns (SetSolved :type Boolean))
  (return false))

(fn `UserConstructionScript`)

(fn `Valid`
  (returns (Interactable :type Boolean) (Typ :type "/Game/01_DEV/Puzzle/E_Interactable_Type Enum"))
  (return (and (`self.Set Valid`) (not (`KismetSystemLibrary.IsValid` (`self.CurrentItem`)))) "NewEnumerator6"))