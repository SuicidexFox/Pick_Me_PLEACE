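; First-person player character handling movement, look, sprint, crouch, interaction, a cyclable held-item inventory and a toggleable smartphone.
; A looping timer line-traces from the camera for Interface_Interactable actors, sending targeted/untargeted messages and animating a crosshair value; Interact messages the current target.
; Inventory items set the held mesh, materials and transform.
; The phone flip-flops a HUD widget with fade and pause timelines, blocking input through CanMove while open.
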(event `self.ReceiveBeginPlay`
  ;[1 1 1] Eigenes Tick-Event
  ; Custom Event/Funktions
  (`KismetSystemLibrary.K2_SetTimer` null "Crosshair" 0.1 true true)
  ;[0.1119 0.4969 0.5906] Crosair Timeline
  (`TimelineComponent.SetPlayRate` (`self.CrosairTimeline`) 5.0))

(event `Crosshair`
  (bind _firstpersoncamera (`self.FirstPersonCamera`))
  (bind _returnvalue (`SceneComponent.K2_GetComponentLocation` _firstpersoncamera))
  ;[1 0.6829 0] Crosshair
  ;;[1 1 1] Gizmo vom Crosshair
  (bind (_outhit _returnvalue_2) (`KismetSystemLibrary.LineTraceSingle` :`Start` _returnvalue :`End` (+ _returnvalue (* (`KismetMathLibrary.Normal` (`SceneComponent.GetForwardVector` _firstpersoncamera)) 150.0)) :`TraceChannel` "TraceTypeQuery1" :`TraceColor` (struct :`R` 0.322784 :`G` 0.309979 :`B` 1.0 :`A` 1.0) :`DrawTime` 1.0)) ; Setzt und Start und Ende des geschossenen Punkts
  ;;[1 1 1] Abfrage vom Interactable
  (if _returnvalue_2
    (bind (_bblockinghit _binitialoverlap _time _distance _location _impactpoint _normal _impactnormal _physmat _hitactor) (`GameplayStatics.BreakHitResult` _outhit))
    (bind _interactable (message `/Game/01_DEV/Interface_and_Self/Interface_Interactable.Valid` _hitactor))
    (if (and _interactable (`KismetSystemLibrary.DoesImplementInterface` _hitactor "/Game/01_DEV/Interface_and_Self/Interface_Interactable.Interface_Interactable_C"))
      (bind _output_get (set `self.CurrentInteractable` _hitactor))
      (message `/Game/01_DEV/Interface_and_Self/Interface_Interactable.Targeted` _output_get)
      (bind (_direction _value) (`Timeline|Anim_Valid` :!label _label)
        (:`Update`
          (set `self.AnimValid` _value)))
      (else
        (message `/Game/01_DEV/Interface_and_Self/Interface_Interactable.Untargeted` _output_get :!label _label_2)
        (set `self.CurrentInteractable` null)
        (goto _label :!via `Reverse`)))
    (else
      (goto _label_2))))

(event `CurrentInventory`
  (params (SetItem :type "/Game/01_DEV/Instruction/Item/ItemStructure Structure"))
  (bind _returnvalue (`KismetArrayLibrary.Array_Add` (`self.Inventory`) SetItem))
  (set `self.CurrentIntemIndex` _returnvalue)
  (`self.ShowItem`)
  (goto _label_2))

(event `ShowItem`
  (bind _itemmesh (`self.ItemMesh`))
  (bind (_name _mesh _materials _transform) (break `/Game/01_DEV/Instruction/Item/ItemStructure` (`|GetArrayItem` (`self.Inventory`) (`self.CurrentIntemIndex`))))
  (if (`KismetStringLibrary.EqualEqual_StrStr` (`.Name_5_1C06FF694E268D40E70FD589ADD5300D` (break `/Game/01_DEV/Instruction/Item/ItemStructure` (`|GetArrayItem` (`self.Inventory`) (`self.CurrentIntemIndex`)))))
    (`SceneComponent.SetVisibility` (`self.ItemMesh`) false false)
    (else
      (`SceneComponent.SetVisibility` (`self.ItemMesh`) true false)
      (`StaticMeshComponent.SetStaticMesh` _itemmesh _mesh)
      (for (_array_element _array_index) _materials
        (`PrimitiveComponent.SetMaterial` _itemmesh _array_index _array_element))
      (`SceneComponent.K2_SetRelativeTransform` (`self.ItemMesh`) _transform false true))))

(event `EnhancedInput|/Game/01_DEV/Input/IA_Interact`
  (params (ActionValue :type Boolean) (ElapsedSeconds :type "Float (double-precision)") (TriggeredSeconds :type "Float (double-precision)") (InputAction :type "InputAction Object Reference" :default "/Game/01_DEV/Input/IA_Interact.IA_Interact"))
  ;[1 0.7758 0.1812] Interactable
  (:`Started`
    (if (`self.CanMove`)
      (bind _currentinteractable (`self.CurrentInteractable`)
        (:`then`
          (message `/Game/01_DEV/Interface_and_Self/Interface_Interactable.Interact` _currentinteractable self))
        (:`else`)))))

(event `EnhancedInput|/Game/01_DEV/Input/IA_Look`
  (params (ActionValue :type "Vector2D Structure") (ElapsedSeconds :type "Float (double-precision)") (TriggeredSeconds :type "Float (double-precision)") (InputAction :type "InputAction Object Reference" :default "/Game/01_DEV/Input/IA_Look.IA_Look"))
  ;[0.2623 0.5906 1] Look
  (:`Triggered`
    (if (`self.CanMove`)
      (`self.AddControllerYawInput` ActionValue_X)
      (`self.AddControllerPitchInput` ActionValue_Y))))

(event `EnhancedInput|/Game/01_DEV/Input/IA_Inventory_For`
  (params (ActionValue :type Boolean) (ElapsedSeconds :type "Float (double-precision)") (TriggeredSeconds :type "Float (double-precision)") (InputAction :type "InputAction Object Reference" :default "/Game/01_DEV/Input/IA_Inventory_For.IA_Inventory_For"))
  ;[1 0.7758 0.1812] Inventory
  (:`Started`
    (if (`self.CanMove`)
      (bind _result (`/Engine/EditorBlueprintResources/StandardMacros.IncrementInt` (`self.CurrentIntemIndex`))
        (:`  `
          (set `self.CurrentIntemIndex` (`KismetMathLibrary.SelectInt` 0 _result (> _result (`KismetArrayLibrary.Array_LastIndex` (`self.Inventory`)))))
          (`self.ShowItem`))))))

(event `EnhancedInput|/Game/01_DEV/Input/IA_Move`
  (params (ActionValue :type "Vector2D Structure") (ElapsedSeconds :type "Float (double-precision)") (TriggeredSeconds :type "Float (double-precision)") (InputAction :type "InputAction Object Reference" :default "/Game/01_DEV/Input/IA_Move.IA_Move"))
  ;[0.2623 0.5906 1] Move
  (:`Triggered`
    (if (`self.CanMove`)
      (`self.AddMovementInput` (`self.GetActorRightVector`) ActionValue_X)
      (`self.AddMovementInput` (`self.GetActorForwardVector`) ActionValue_Y))))

(event `EnhancedInput|/Game/01_DEV/Input/IA_Sprint`
  (params (ActionValue :type Boolean) (ElapsedSeconds :type "Float (double-precision)") (TriggeredSeconds :type "Float (double-precision)") (InputAction :type "InputAction Object Reference" :default "/Game/01_DEV/Input/IA_Sprint.IA_Sprint"))
  ;[0.2623 0.5906 1] Comment
  (:`Triggered`
    (if (`self.CanMove`)
      (set `CharacterMovementComponent.MaxWalkSpeed` 350.0 (`self.CharacterMovement`))))
  (:`Completed`
    (set `CharacterMovementComponent.MaxWalkSpeed` 200.0 (`self.CharacterMovement`))))

(event `EnhancedInput|/Game/01_DEV/Input/IA_Crouch`
  (params (ActionValue :type Boolean) (ElapsedSeconds :type "Float (double-precision)") (TriggeredSeconds :type "Float (double-precision)") (InputAction :type "InputAction Object Reference" :default "/Game/01_DEV/Input/IA_Crouch.IA_Crouch"))
  ;[0.2623 0.5906 1] Crouch
  (:`Triggered`
    (if (`self.CanMove`)
      (`self.Crouch`)))
  (:`Completed`
    (`self.UnCrouch`)))

(event `EnhancedInput|/Game/01_DEV/Input/IA_Inventory_Back`
  (params (ActionValue :type Boolean) (ElapsedSeconds :type "Float (double-precision)") (TriggeredSeconds :type "Float (double-precision)") (InputAction :type "InputAction Object Reference" :default "/Game/01_DEV/Input/IA_Inventory_Back.IA_Inventory_Back"))
  ;[1 0.7758 0.1812] Inventory
  (:`Started`
    (if (`self.CanMove`)
      (bind _result (`/Engine/EditorBlueprintResources/StandardMacros.DecrementInt` (`self.CurrentIntemIndex`))
        (:`  `
          (set `self.CurrentIntemIndex` (`KismetMathLibrary.SelectInt` (`KismetArrayLibrary.Array_LastIndex` (`self.Inventory`)) _result (< _result 0)))
          (`self.ShowItem`))))))

(event `EnhancedInput|/Game/01_DEV/Input/IA_Phone`
  (params (ActionValue :type Boolean) (ElapsedSeconds :type "Float (double-precision)") (TriggeredSeconds :type "Float (double-precision)") (InputAction :type "InputAction Object Reference" :default "/Game/01_DEV/Input/IA_Phone.IA_Phone"))
  (bind _widget_smartphone (`self.Widget_Smartphone`))
  (bind (_crosair_stack _smartphone_stack) (`/Game/01_DEV/Interface_and_Self/FL_Utils.GetHUD_PMP` (`GameplayStatics.GetPlayerController` 0)))
  ;[1 1 1] Q - ShowSmartphone
  (:`Started`
    (if (`self.CanMove`)
      (if (not (`self.Ring`))
        (if (not (`self.Animation`))
          (set `self.Animation` true)
          (`/Engine/EditorBlueprintResources/StandardMacros.FlipFlop`
            (:`A`
              (set `self.CanMove` false)
              (bind _returnvalue (`CommonActivatableWidgetContainerBase.BP_AddWidget` _smartphone_stack "/Game/02_UI/Smartphone/AWB_Smartphone.AWB_Smartphone_C"))
              (bind _output_get (set `self.Widget_Smartphone` _returnvalue))
              (`UserWidget.PlayAnimationForward` _output_get (`/Game/02_UI/Smartphone/AWB_Smartphone.Anim_Fade` _output_get) 1.0 false)
              (bind (_direction _value) (`Timeline|Anim_Pause` :!label _label)
                (:`Update`
                  (set `self.AnimPause` _value)
                  (`KismetSystemLibrary.Delay` 1.0)
                  (set `self.Animation` false))))
            (:`B`
              (`UserWidget.PlayAnimationReverse` _widget_smartphone (`/Game/02_UI/Smartphone/AWB_Smartphone.Anim_Fade` _widget_smartphone) 1.0 false)
              (`|ExecutionSequence`
                (:`then_0`
                  (goto _label :!via `Reverse`))
                (:`then_1`
                  (`KismetSystemLibrary.Delay` 1.0)
                  (set `self.Animation` false)
                  (`CommonActivatableWidgetContainerBase.RemoveWidget` _smartphone_stack (`self.Widget_Smartphone`))
                  (`WidgetBlueprintLibrary.SetInputMode_GameOnly` (`GameplayStatics.GetPlayerController` 0))
                  (set `self.CanMove` true))))))))))

(fn `UserConstructionScript`)