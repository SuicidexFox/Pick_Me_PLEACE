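; BP_BeginPlay is an interactable Blueprint whose Interact event plays a camera fade-out and fade-in on the first player's camera manager.
; The event fades the screen out, waits for the fade to finish, then fades back in from black.
; SetSolved always returns false, and Valid reports it as non-interactable with a fixed type.
; Possession calls, both smooth and direct, remain in the graph but are disconnected.
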(event `/Game/01_DEV/Interactables/Interface_Interactable.Interact`
  (params (Player_ID :type "/Game/01_DEV/BP_Player Object Reference"))
  (bind _returnvalue (`GameplayStatics.GetPlayerCameraManager` 0))
  (`PlayerCameraManager.StartCameraFade` :`self` _returnvalue :`ToAlpha` 1.0 :`Duration` 0.5)
  (`KismetSystemLibrary.Delay` 0.5)
  (`PlayerCameraManager.StartCameraFade` _returnvalue 1.0 0.0 0.5 (struct :`A` 1.0) false false))

(fn `SetSolved`
  (returns (SetSolved :type Boolean))
  (return false))

(fn `UserConstructionScript`)

(fn `Valid`
  (returns (Interactable :type Boolean) (Typ :type "/Game/01_DEV/Interactables/E_Interactable_Type Enum"))
  (return false "NewEnumerator4"))