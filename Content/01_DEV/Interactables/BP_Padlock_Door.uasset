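; BP_Padlock_Door is an interactable padlocked double door that opens when its lock is solved.
; On the Solved event, a sequence starts two one-second MoveComponentTo calls that swing the left and right door components to opposite yaw rotations.
; The SetSolved function returns false, and Valid reports the door as non-interactable along with a fixed type enum.
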(event `/Game/01_DEV/Interface_and_Self/Interface_Interactable.Solved`
  (bind _lock_door_door_left (`self.Lock_Door_Door_Left`))
  (bind _lock_door_door_right (`self.Lock_Door_Door_Right`))
  (`|ExecutionSequence`
    (:`then_0`
      (`KismetSystemLibrary.MoveComponentTo` _lock_door_door_left (`SceneComponent.RelativeLocation` _lock_door_door_left) (struct :`Yaw` -80.0) false false 1.0))
    (:`then_1`
      (`KismetSystemLibrary.MoveComponentTo` _lock_door_door_right (`SceneComponent.RelativeLocation` _lock_door_door_right) (struct :`Yaw` 80.0) false false 1.0))))

(fn `SetSolved`
  (returns (SetSolved :type Boolean))
  (return false))

(fn `UserConstructionScript`)

(fn `Valid`
  (returns (Interactable :type Boolean) (Typ :type "/Game/01_DEV/Interactables/E_Interactable_Type Enum"))
  (return false "NewEnumerator4"))