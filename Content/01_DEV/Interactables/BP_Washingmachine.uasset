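; Washing machine interactable that puts the player into an inspect view and slides out its drawer.
; Interact saves the control rotation, locks movement, smooth-possesses the machine, fades in an inspect widget on the HUD crosshair stack and moves the drawer.
; Tab reverses the drawer and fade, possesses the player again, then restores rotation and movement.
; Puzzle logic is unfinished: SetSolved returns false, the StocksCorrect check is unconnected and the interact input is empty.
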(event `/Game/01_DEV/Interface_and_Self/Interface_Interactable.Interact`
  (params (Player_ID :type "/Game/01_DEV/BP_Player Object Reference"))
  (bind _washingmachine_auszug (`self.Washingmachine_Auszug`))
  (bind _output_get (set `self.PlayerID` Player_ID))
  (set `self.PlayerControllerRotation` (`self.GetControlRotation` _output_get))
  (set `/Game/01_DEV/BP_Player.CanMove` false _output_get)
  (`|ExecutionSequence`
    (:`then_0`
      (`/Game/01_DEV/Interface_and_Self/ML_Utils.SmothPossess` (`GameplayStatics.GetPlayerController` 0) self
        (:`then`
          ;[1 1 1] Widget
          (bind _returnvalue (`CommonActivatableWidgetContainerBase.BP_AddWidget` (`/Game/01_DEV/Interface_and_Self/FL_Utils.GetHUD_PMP` (`GameplayStatics.GetPlayerController` 0)) "/Game/02_UI/Controls/AWB_Inspacted.AWB_Inspacted_C"))
          (bind _output_get_2 (set `self.CurrentWidget` _returnvalue))
          (`UserWidget.PlayAnimationForward` _output_get_2 (`/Game/02_UI/Controls/AWB_Inspacted.Anim_Opacity` _output_get_2) 1.0 false))))
    (:`then_1`
      ;[1 1 1] Auszug
      (`KismetSystemLibrary.MoveComponentTo` _washingmachine_auszug (+ (`SceneComponent.RelativeLocation` _washingmachine_auszug) (-11.0 0.0 0.0)) (`SceneComponent.RelativeRotation` _washingmachine_auszug) true true 1.0))))

(event `EnhancedInput|/Game/01_DEV/Input/IA_Tab`
  (params (ActionValue :type Boolean) (ElapsedSeconds :type "Float (double-precision)") (TriggeredSeconds :type "Float (double-precision)") (InputAction :type "InputAction Object Reference" :default "/Game/01_DEV/Input/IA_Tab.IA_Tab"))
  (bind _returnvalue (`GameplayStatics.GetPlayerController` 0))
  (bind _currentwidget (`self.CurrentWidget`))
  (bind _playerid (`self.PlayerID`))
  (bind _washingmachine_auszug (`self.Washingmachine_Auszug`))
  ;[1 1 1] Laeve
  (:`Started`
    (`/Game/01_DEV/Interface_and_Self/ML_Utils.SmothPossess` _returnvalue _playerid
      (:`Compledet`
        (`Controller.SetControlRotation` _returnvalue (`self.PlayerControllerRotation`))
        (set `/Game/01_DEV/BP_Player.CanMove` true _playerid)
        (`CommonActivatableWidgetContainerBase.RemoveWidget` (`/Game/01_DEV/Interface_and_Self/FL_Utils.GetHUD_PMP` (`GameplayStatics.GetPlayerController` 0)) (`self.CurrentWidget`)))
      (:`then`
        (`UserWidget.PlayAnimationReverse` _currentwidget (`/Game/02_UI/Controls/AWB_Inspacted.Anim_Opacity` _currentwidget) 1.0 false)
        (`KismetSystemLibrary.MoveComponentTo` _washingmachine_auszug (- (`SceneComponent.RelativeLocation` _washingmachine_auszug) (-11.0 0.0 0.0)) (`SceneComponent.RelativeRotation` _washingmachine_auszug) true true 1.0)))))

(event `EnhancedInput|/Game/01_DEV/Input/IA_Interact`
  (params (ActionValue :type Boolean) (ElapsedSeconds :type "Float (double-precision)") (TriggeredSeconds :type "Float (double-precision)") (InputAction :type "InputAction Object Reference" :default "/Game/01_DEV/Input/IA_Interact.IA_Interact")))

(fn `SetSolved`
  (returns (SetSolved :type Boolean))
  (return false))

(fn `UserConstructionScript`)

(fn `Valid`
  (returns (Interactable :type Boolean) (Typ :type "/Game/01_DEV/Interactables/E_Interactable_Type Enum"))
  (return (`self.IsInteractable`) (`self.Typ`)))