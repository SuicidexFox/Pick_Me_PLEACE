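; BP_Item_Stocking is an interactable stocking item that reports its interactable state and type through Valid.
; Interact checks whether the player's current inventory item is named "Basket", then loops over the PuzzleManager's PuzzleToCheck list with an empty body.
; SetValid stores the flag that Valid returns, while SetSolved always returns false.
; The logic looks unfinished, as a DestroyActor call is left unconnected.
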(event `self.Interact`
  (params (Player_ID :type "/Game/01_DEV/BP_Player Object Reference"))
  (if (`KismetStringLibrary.EqualEqual_StrStr` (`.Name_5_1C06FF694E268D40E70FD589ADD5300D` (break `/Game/01_DEV/Interactables/ItemStructure` (`|GetArrayItem` (`/Game/01_DEV/BP_Player.Inventory` Player_ID) (`/Game/01_DEV/BP_Player.CurrentIntemIndex` Player_ID)))) "Basket")
    (for _ (`/Game/01_DEV/Instruction/BP_PuzzleManager.PuzzleToCheck` (`self.PuzzleManager`))
      _)))

(event `self.SetValid`
  (params (SetValid :type Boolean))
  (set `self.Set Valid` SetValid))

(fn `SetSolved`
  (returns (SetSolved :type Boolean))
  (return false))

(fn `UserConstructionScript`)

(fn `Valid`
  (returns (Interactable :type Boolean) (Typ :type "/Game/01_DEV/Interactables/E_Interactable_Type Enum"))
  (return (`self.Set Valid`) "NewEnumerator0"))