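; Interactable calendar pawn that the player can pick up to inspect and rotate, with empty solved/unsolved puzzle events.
; Interact snaps its camera to the player's first-person view, pushes an inspect widget, possesses the pawn and eases the calendar in front of the camera.
; Move input either yaws the whole scene or flips the mesh within a clamped roll range.
; Interacting again returns the calendar, restores player possession and view rotation, and removes the widget.
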(event `self.ReceiveBeginPlay`
  (set `self.StartTransform` (`SceneComponent.GetRelativeTransform` (`self.Scene`))))

(event `self.Interact`
  (params (Player_ID :type "/Game/01_DEV/BP_Player_0 Object Reference"))
  (bind _returnvalue (`GameplayStatics.GetPlayerController` 0))
  (bind _camera (`self.Camera`))
  (bind _returnvalue_2 (`SceneComponent.GetRelativeTransform` _camera))
  ;[1 1 1] Interact
  (`|ExecutionSequence`
    (:`then_0`
      (bind _output_get (set `self.Player ID` Player_ID))
      (bind (_returnvalue_location _returnvalue_rotation) (`KismetMathLibrary.BreakTransform` (`SceneComponent.K2_GetComponentToWorld` (`/Game/01_DEV/BP_Player_0.FirstPersonCamera` _output_get))))
      ;;[1 0.4852 0.05286] Cam Bewegt sich zu unserer Cam
      (`SceneComponent.K2_SetWorldLocationAndRotation` (`self.Camera`) _returnvalue_location _returnvalue_rotation true false)
      (bind _returnvalue_3 (`CommonActivatableWidgetContainerBase.BP_AddWidget` (`/Game/01_DEV/FL_Utils.Set Up Widget Stack` (`GameplayStatics.GetPlayerController` 0)) "/Game/02_UI/Activateble_Widget_Inspacted.Activateble_Widget_Inspacted_C"))
      (bind _output_get_2 (set `self.CurrentWidget` _returnvalue_3))
      (`UserWidget.QueuePlayAnimationForward` _output_get_2 (`/Game/02_UI/Activateble_Widget_Inspacted.Anim_Opacity` _output_get_2) 1.0 false))
    (:`then_1`
      (set `self.PlayerControllerRotation` (`Controller.GetControlRotation` _returnvalue))
      (`Controller.Possess` _returnvalue self) ; Inputs werden\nPawn übergeben
    )
    (:`then_2`
      ;;[1 0.4852 0.05286] Scene bewegt sich vor unsere Camera
      (`KismetSystemLibrary.MoveComponentTo` (`self.Scene`) (+ (`KismetMathLibrary.MakeVector` (.x (.location _returnvalue_2)) (.y (.location _returnvalue_2)) (`self.High`)) (* (`KismetMathLibrary.Normal` (`SceneComponent.GetForwardVector` _camera)) (`self.Distance`))) (.rotation _returnvalue_2) true true 1.0)
      (set `self.IsInspacted` true))))

(event `/Game/01_DEV/Interactables/Interface_Interactable.Solved`)

(event `/Game/01_DEV/Interactables/Interface_Interactable.Unsolved`)

(event `EnhancedInput|/Game/01_DEV/Input/IA_Interact`
  (params (ActionValue :type Boolean) (ElapsedSeconds :type "Float (double-precision)") (TriggeredSeconds :type "Float (double-precision)") (InputAction :type "InputAction Object Reference" :default "/Game/01_DEV/Input/IA_Interact.IA_Interact"))
  (bind _returnvalue (`GameplayStatics.GetPlayerController` 0))
  (bind (_starttransform_location _starttransform_rotation) (`KismetMathLibrary.BreakTransform` (`self.StartTransform`)))
  (bind _currentwidget (`self.CurrentWidget`))
  (bind _movablemesh (`self.MovableMesh`))
  (bind (_relativerotation_roll _relativerotation_pitch _relativerotation_yaw) (`KismetMathLibrary.BreakRotator` (`SceneComponent.RelativeRotation` _movablemesh)))
  ;[1 1 1] Leave
  (:`Started`
    (`|ExecutionSequence`
      (:`then_0`
        (if (`self.IsInspacted`)
          (set `self.IsInspacted` false)
          ;;[1 0.4852 0.05286] Scene move to Start
          (`KismetSystemLibrary.MoveComponentTo` (`self.Scene`) _starttransform_location _starttransform_rotation true true 1.0)
          (`Controller.Possess` _returnvalue (`self.Player ID`))
          (`Controller.SetControlRotation` _returnvalue (`self.PlayerControllerRotation`))
          (`CommonActivatableWidgetContainerBase.RemoveWidget` (`/Game/01_DEV/FL_Utils.Set Up Widget Stack` _returnvalue) (`self.CurrentWidget`))))
      (:`then_1`
        (`KismetSystemLibrary.MoveComponentTo` _movablemesh (0.0 0.0 0.0) (`KismetMathLibrary.MakeRotator` 0.0 _relativerotation_pitch _relativerotation_yaw) true true 1.0))
      (:`then_2`
        (`UserWidget.PlayAnimationReverse` _currentwidget (`/Game/02_UI/Activateble_Widget_Inspacted.Anim_Opacity` _currentwidget) 1.0 false)))))

(event `EnhancedInput|/Game/01_DEV/Input/IA_Move`
  (params (ActionValue :type "Vector2D Structure") (ElapsedSeconds :type "Float (double-precision)") (TriggeredSeconds :type "Float (double-precision)") (InputAction :type "InputAction Object Reference" :default "/Game/01_DEV/Input/IA_Move.IA_Move"))
  (bind (_returnvalue_roll _returnvalue_pitch) (`KismetMathLibrary.BreakRotator` (`KismetMathLibrary.MakeRotator` 0.0 (* ActionValue_Y -4.0))))
  (bind (_returnvalue_roll_2 _returnvalue_pitch_2) (`KismetMathLibrary.BreakRotator` (`KismetMathLibrary.MakeRotator` 0.0 (* ActionValue_X -4.0))))
  ;[1 1 1] Moveable
  (:`Triggered`
    (if (< (`KismetMathLibrary.Abs` ActionValue_X) (`KismetMathLibrary.Abs` ActionValue_Y))
      (`SceneComponent.K2_AddLocalRotation` (`self.MovableMesh`) (`KismetMathLibrary.MakeRotator` _returnvalue_pitch) false true)
      (`self.StopRotation`)
      (else
        (`SceneComponent.K2_AddLocalRotation` (`self.Scene`) (`KismetMathLibrary.MakeRotator` 0.0 0.0 _returnvalue_pitch_2) false true)))))

(fn `SetSolved`
  (returns (IsSolved :type Boolean))
  (return false))

(fn `StopRotation`
  (bind _movablemesh (`self.MovableMesh`))
  (bind (_relativerotation_roll _relativerotation_pitch _relativerotation_yaw) (`KismetMathLibrary.BreakRotator` (`SceneComponent.RelativeRotation` _movablemesh)))
  (`|ExecutionSequence`
    (:`then_0`
      (if (> _relativerotation_roll 0.0)
        (`SceneComponent.K2_SetRelativeRotation` _movablemesh (`KismetMathLibrary.MakeRotator` 0.0 _relativerotation_pitch _relativerotation_yaw) false false)))
    (:`then_1`
      (if (< _relativerotation_roll -140.0)
        (`SceneComponent.K2_SetRelativeRotation` _movablemesh (`KismetMathLibrary.MakeRotator` -140.0 _relativerotation_pitch _relativerotation_yaw) false false)))))

(fn `UserConstructionScript`)

(fn `Valid`
  (returns (IsInteractable :type Boolean) (Typ :type "/Game/01_DEV/Interactables/E_Interactable_Type Enum"))
  (return (`self.IsInteractable`) (`self.Typ`)))