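; Laundry basket pickup that moves itself into the interacting player's inventory.
; On Interact it packs its ID, mesh, materials, transform with scaled-down size, and class into an item structure passed to the player's CurrentInventory.
; It then sends a valid message to every linked ActortoReact entry and destroys itself.
; Valid reports interactability from SetValid with a fixed type, while SetSolved always returns false.
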(event `/Game/01_DEV/Interface_and_Self/Interface_Interactable.Interact`
  (params (Player_ID :type "/Game/01_DEV/BP_Player Object Reference"))
  (bind _basket (`self.Basket`))
  (`/Game/01_DEV/BP_Player.CurrentInventory` Player_ID (make `/Game/01_DEV/Interactables/ItemStructure` null (`self.ItemID`) (`StaticMeshComponent.StaticMesh` _basket) (`MeshComponent.GetMaterials` _basket) (`KismetMathLibrary.MakeTransform` (`SceneComponent.RelativeLocation` _basket) (`SceneComponent.RelativeRotation` _basket) (/ (`SceneComponent.K2_GetComponentScale` _basket) (2.5 2.5 2.5))) (`GameplayStatics.GetObjectClass` self)))
  (for _array_element (`self.ActortoReact`)
    (message `/Game/01_DEV/Interface_and_Self/Interface_Interactable.SetValid` _array_element true))
  (`self.K2_DestroyActor`))

(fn `SetSolved`
  (returns (SetSolved :type Boolean))
  (return false))

(fn `UserConstructionScript`)

(fn `Valid`
  (returns (Interactable :type Boolean) (Typ :type "/Game/01_DEV/Interactables/E_Interactable_Type Enum"))
  (return (`self.Set Valid`) "NewEnumerator0"))