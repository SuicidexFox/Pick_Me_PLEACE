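; BP_ItemSocket is an interactable socket where the player places the selected inventory item.
; Interact spawns that item at the socket, removes it from inventory and refreshes the held item, or shows a monologue line when none is selected.
; A NeedItem match also retypes the spawned item through a Rub cast.
; The socket is interactable only while enabled and empty; its solved-notification logic is disconnected.
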(event `/Game/01_DEV/Interface_and_Self/Interface_Interactable.Interact`
  (params (Player_ID :type "/Game/01_DEV/BP_Player Object Reference"))
  (bind _inventory (`/Game/01_DEV/BP_Player.Inventory` Player_ID))
  (bind _currentintemindex (`/Game/01_DEV/BP_Player.CurrentIntemIndex` Player_ID))
  (bind (_name _mesh _materials _transform _class) (break `/Game/01_DEV/Interactables/Items/ItemStructure` (`|GetArrayItem` _inventory _currentintemindex)))
  (if (`KismetStringLibrary.NotEqual_StrStr` _name)
    (`self.CurrentItem`
      (:`then`)
      (:`else`
        (bind _returnvalue (`|SpawnActorFromClass` _class (`SceneComponent.K2_GetComponentToWorld` (`self.Scene`)) "Undefined" "MultiplyWithRoot" null null))
        (bind _output_get (set `self.CurrentItem` _returnvalue))
        (if (`KismetStringLibrary.EqualEqual_StrStr` (`self.NeedItem`) _name)
          (bind _asrub (cast `/Game/01_DEV/Interactables/Items/Rub` _output_get))
          (set `/Game/01_DEV/Interactables/Items/BP_Item.Typ` "NewEnumerator3" _asrub))
        (`KismetArrayLibrary.Array_Remove` _inventory _currentintemindex)
        (`/Game/01_DEV/BP_Player.ShowItem` Player_ID)))
    (else
      (`/Game/01_DEV/Interface_and_Self/FL_Utils.SetNewSelfMonolog` (`GameplayStatics.GetPlayerController` 0) "Forward" "Mir fehlt noch etwas"))))

(event `/Game/01_DEV/Interface_and_Self/Interface_Interactable.SetValid`
  (params (SetValid :type Boolean))
  (bind _output_get (set `self.SetInteractable` SetValid))
  (message `/Game/01_DEV/Interface_and_Self/Interface_Interactable.SetValid` (`self.CurrentItem`) _output_get))

(fn `SetSolved`
  (returns (SetSolved :type Boolean))
  (return (`self.Set Solved`)))

(fn `UserConstructionScript`)

(fn `Valid`
  (returns (Interactable :type Boolean) (Typ :type "/Game/01_DEV/Interactables/E_Interactable_Type Enum"))
  (return (and (`self.SetInteractable`) (not (`KismetSystemLibrary.IsValid` (`self.CurrentItem`)))) "NewEnumerator6"))