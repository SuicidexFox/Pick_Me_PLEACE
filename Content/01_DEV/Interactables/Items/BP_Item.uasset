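; BP_Item is an interactable item that a player picks up.
; On Interact it packs its name, mesh, materials, transform and class into an item structure and passes it to that player's CurrentInventory.
; It then sends SetValidMessage to every actor in ActortoReact and destroys itself.
; Valid reports the SetValid flag with a fixed type, and SetSolved always returns false.
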(event `/Game/01_DEV/Interface_and_Self/Interface_Interactable.Interact`
  (params (Player_ID :type "/Game/01_DEV/BP_Player Object Reference"))
  (bind _mesh (`self.Mesh`))
  (`/Game/01_DEV/BP_Player.CurrentInventory` Player_ID (make `/Game/01_DEV/Interactables/Items/ItemStructure` (`KismetSystemLibrary.GetDisplayName` self) (`StaticMeshComponent.StaticMesh` _mesh) (`MeshComponent.GetMaterials` _mesh) (`KismetMathLibrary.MakeTransform` (`SceneComponent.RelativeLocation` _mesh) (`SceneComponent.RelativeRotation` _mesh) (`SceneComponent.K2_GetComponentScale` _mesh)) (`GameplayStatics.GetObjectClass` self)))
  (for _array_element (`self.ActortoReact`)
    (message `/Game/01_DEV/Interface_and_Self/Interface_Interactable.SetValid` _array_element true))
  (`self.K2_DestroyActor`))

(fn `SetSolved`
  (returns (SetSolved :type Boolean))
  (return false))

(fn `UserConstructionScript`)

(fn `Valid`
  (returns (Interactable :type Boolean) (Typ :type "/Game/01_DEV/Interactables/E_Interactable_Type Enum"))
  (return (`self.Set Valid`) "NewEnumerator0"))