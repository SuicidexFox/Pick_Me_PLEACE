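; Interactable right-hand wardrobe door that takes over control from the player and animates open.
; On interact it caches the player and control rotation, disables their movement, smooth-possesses itself and moves the door sideways while swinging it over one second.
; Solved and the Tab input share a move that rotates the door to the same angle at its current location, without handing control back.
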(event `/Game/01_DEV/Interface_and_Self/Interface_Interactable.Interact`
  (params (Player_ID :type "/Game/01_DEV/BP_Player Object Reference"))
  (bind _wardrobe_door_r (`self.Wardrobe_Door_r`))
  (bind _output_get (set `self.Player` Player_ID))
  (set `self.PlayerRotation` (`self.GetControlRotation` _output_get))
  (set `/Game/01_DEV/BP_Player.CanMove` false _output_get)
  (`/Game/01_DEV/Interface_and_Self/ML_Utils.SmothPossess` (`GameplayStatics.GetPlayerController` 0) self
    (:`then`
      (bind _output_get_2 (set `self.StartLocation` (`SceneComponent.RelativeLocation` _wardrobe_door_r)))
      (`KismetSystemLibrary.MoveComponentTo` _wardrobe_door_r (`KismetMathLibrary.MakeVector` (.x _output_get_2) 90.0 (.z _output_get_2)) (struct :`Yaw` -80.0) false false 1.0))))

(event `self.Solved`
  (bind _wardrobe_door_r (`self.Wardrobe_Door_r`))
  (`KismetSystemLibrary.MoveComponentTo` _wardrobe_door_r (`SceneComponent.RelativeLocation` _wardrobe_door_r) (struct :`Yaw` -80.0) false false 1.0 :!label _label))

(event `EnhancedInput|/Game/01_DEV/Input/IA_Tab`
  (params (ActionValue :type Boolean) (ElapsedSeconds :type "Float (double-precision)") (TriggeredSeconds :type "Float (double-precision)") (InputAction :type "InputAction Object Reference" :default "/Game/01_DEV/Input/IA_Tab.IA_Tab"))
  (:`Started`
    (goto _label)))

(fn `SetSolved`
  (returns (SetSolved :type Boolean))
  (return false))

(fn `UserConstructionScript`)

(fn `Valid`
  (returns (Interactable :type Boolean) (Typ :type "/Game/01_DEV/Interactables/E_Interactable_Type Enum"))
  (return (`self.Interactable`) "NewEnumerator2"))