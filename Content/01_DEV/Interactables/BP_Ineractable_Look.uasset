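; Interactable three-wheel combination lock that takes over the player's view through a smooth possess and shows an inspection widget.
; Move input cycles the overlay-highlighted wheel or rolls it one step, and Interact hands control back.
; After each roll, SetupSolved records wheel angles, but its check is hard-wired true, so it opens the shackle and notifies ActorToReact actors once without comparing a combination.
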(event `self.ReceiveBeginPlay`
  ;[1 1 1] Whells
  (set `self.ListWheel` (`|MakeArray` (`self.Wheel1`) (`self.Wheel2`) (`self.Wheel3`))))

(event `/Game/01_DEV/Interactables/Interface_Interactable.Interact`
  (params (Player_ID :type "/Game/01_DEV/BP_Player Object Reference"))
  (bind _output_get (set `self.Player ID` Player_ID))
  (set `self.PlayerControllerRotation` (`self.GetControlRotation` _output_get))
  (set `/Game/01_DEV/BP_Player.CanMove` false _output_get)
  (`/Game/01_DEV/ML_Utils.SmothPossess` (`GameplayStatics.GetPlayerController` 0) self
    (:`Completed`
      (set `self.IsInspacted` true)
      (`MeshComponent.SetOverlayMaterial` (`self.CurrentWheel`) "/Game/04_Material/MI_Shader_Smal.MI_Shader_Smal")
      ;[1 1 1] Widget
      (bind _returnvalue (`CommonActivatableWidgetContainerBase.BP_AddWidget` (`/Game/01_DEV/FL_Utils.Set Up Widget Stack` (`GameplayStatics.GetPlayerController` 0)) "/Game/02_UI/Controls/AWB_Inspacted.AWB_Inspacted_C"))
      (bind _output_get_2 (set `self.CurrentWidget` _returnvalue))
      (`UserWidget.PlayAnimationForward` _output_get_2 (`/Game/02_UI/Controls/AWB_Inspacted.Anim_Opacity` _output_get_2) 1.0 false))))

(event `SetupSolved`
  (for (_array_element _array_index) (`self.ListWheel`)
    (bind _relativerotation_roll (`KismetMathLibrary.BreakRotator` (`SceneComponent.RelativeRotation` _array_element)))
    (`KismetArrayLibrary.Array_Set` (`self.CurrentX`) _array_index _relativerotation_roll)
    (if true
      (`/Engine/EditorBlueprintResources/StandardMacros.DoOnce` false
        (:`Completed`
          (`KismetSystemLibrary.MoveComponentTo` (`self.Shackle`) (0.0 0.0 0.0) (struct :`Pitch` -50.0) true true 1.0)
          (for _array_element_2 (`self.ActorToReact`)
            (message `/Game/01_DEV/Interactables/Interface_Interactable.Solved` _array_element_2))))
      (else
        (`self.ResetInput`)))))

(event `EnhancedInput|/Game/01_DEV/Input/IA_Interact`
  (params (ActionValue :type Boolean) (ElapsedSeconds :type "Float (double-precision)") (TriggeredSeconds :type "Float (double-precision)") (InputAction :type "InputAction Object Reference" :default "/Game/01_DEV/Input/IA_Interact.IA_Interact"))
  (bind _returnvalue (`GameplayStatics.GetPlayerController` 0))
  (bind _currentwidget (`self.CurrentWidget`))
  (bind _player_id (`self.Player ID`))
  ;[1 1 1] Laeve
  (:`Started`
    (if (`self.IsInspacted`)
      (set `self.IsInspacted` false)
      (`/Game/01_DEV/ML_Utils.SmothPossess` _returnvalue _player_id
        (:`Completed`
          (`Controller.SetControlRotation` _returnvalue (`self.PlayerControllerRotation`))
          (set `/Game/01_DEV/BP_Player.CanMove` true _player_id)
          (`CommonActivatableWidgetContainerBase.RemoveWidget` (`/Game/01_DEV/FL_Utils.Set Up Widget Stack` (`GameplayStatics.GetPlayerController` 0)) (`self.CurrentWidget`)))
        (:`then`
          (`MeshComponent.SetOverlayMaterial` (`self.CurrentWheel`) null)
          (`UserWidget.PlayAnimationReverse` _currentwidget (`/Game/02_UI/Controls/AWB_Inspacted.Anim_Opacity` _currentwidget) 1.0 false))))))

(event `EnhancedInput|/Game/01_DEV/Input/IA_Move`
  (params (ActionValue :type "Vector2D Structure") (ElapsedSeconds :type "Float (double-precision)") (TriggeredSeconds :type "Float (double-precision)") (InputAction :type "InputAction Object Reference" :default "/Game/01_DEV/Input/IA_Move.IA_Move"))
  ;[0.4072 0.3185 0.08022] WASD Abfrage
  (:`Started`
    (`/Engine/EditorBlueprintResources/StandardMacros.DoOnce` false :!label _label
      (:`Completed`
        (if (> (`KismetMathLibrary.Abs` ActionValue_X) (`KismetMathLibrary.Abs` ActionValue_Y))
          (`self.Left/Right` ActionValue_X)
          (else
            (`self.Up/Down` ActionValue_Y)))))))

(event `ResetInput`
  ;[0.4072 0.3185 0.08022] WASD Abfrage
  (goto _label :!via `Reset`))

(event `Left/Right`
  (params (x :type "Float (double-precision)"))
  (bind _currentwheel (`self.CurrentWheel`))
  (bind _arraywheel (`self.ArrayWheel`))
  ;[0.4072 0.3185 0.08022] WASD Abfrage
  ;;[1 0.7781 0.1968] Right/Left
  (if (> x 0.0)
    (`MeshComponent.SetOverlayMaterial` _currentwheel null)
    (`KismetSystemLibrary.Delay` 0.2)
    (`/Engine/EditorBlueprintResources/StandardMacros.IncrementInt` _arraywheel
      (:`  `
        _))
    (else
      (`MeshComponent.SetOverlayMaterial` _currentwheel null)
      (`KismetSystemLibrary.Delay` 0.2)
      (`/Engine/EditorBlueprintResources/StandardMacros.DecrementInt` _arraywheel
        (:`  `
          _))))
  (`self.Loop`)
  (`MeshComponent.SetOverlayMaterial` (`self.CurrentWheel`) "/Game/04_Material/MI_Shader_Smal.MI_Shader_Smal")
  (`self.ResetInput`))

(event `Up/Down`
  (params (y :type "Float (double-precision)"))
  (bind _currentwheel (`self.CurrentWheel`))
  (bind _currentwheel_2 (`self.CurrentWheel`))
  (bind _relativerotation_roll (`KismetMathLibrary.BreakRotator` (`SceneComponent.RelativeRotation` _currentwheel_2)))
  (bind _relativerotation_roll_2 (`KismetMathLibrary.BreakRotator` (`SceneComponent.RelativeRotation` _currentwheel)))
  ;[0.4072 0.3185 0.08022] WASD Abfrage
  ;;[1 0.7602 0.1816] Up/Down
  (if (> y 0.1)
    (`KismetSystemLibrary.MoveComponentTo` _currentwheel (`SceneComponent.RelativeLocation` _currentwheel) (`KismetMathLibrary.MakeRotator` (+ _relativerotation_roll_2 36.0)))
    (else
      (`KismetSystemLibrary.MoveComponentTo` _currentwheel_2 (`SceneComponent.RelativeLocation` _currentwheel_2) (`KismetMathLibrary.MakeRotator` (- _relativerotation_roll 36.0)))))
  (`self.SetupSolved`))

(fn `Loop`
  (bind _arraywheel (`self.ArrayWheel`))
  (if (== _arraywheel 3)
    (set `self.ArrayWheel` 0)
    (elif (== _arraywheel -1)
      (set `self.ArrayWheel` 2)))
  (set `self.CurrentWheel` (`|GetArrayItem` (`self.ListWheel`) (`self.ArrayWheel`))))

(fn `SetSolved`
  (returns (SetSolved :type Boolean))
  (return (`self.IsSolved`)))

(fn `UserConstructionScript`
  (set `self.CurrentWheel` (`self.Wheel1`)))

(fn `Valid`
  (returns (Interactable :type Boolean) (Typ :type "/Game/01_DEV/Interactables/E_Interactable_Type Enum"))
  (return (`self.IsInteractable`) (`self.Typ`)))