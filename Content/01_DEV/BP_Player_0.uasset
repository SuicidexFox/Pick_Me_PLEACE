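; First-person player Blueprint handling look, movement, interaction and an unfinished held-item inventory.
; A looping timer, used instead of Tick, runs a short camera trace that caches CurrentInteractable and plays or reverses a timeline driving the crosshair's Material Parameter Collection.
; Interact input sends InteractMessage to that cached actor, with all input gated by CanMove.
; CurrentInventory stores items and calls ShowItem, which currently always hides the item mesh.
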(event `self.ReceiveBeginPlay`
  ;[1 1 1] Eigenes Tick-Event
  ; Custom Event/Funktions
  (`KismetSystemLibrary.K2_SetTimer` null "Crosshair" 0.1 true true)
  ;[0.1119 0.4969 0.5906] Crosair Timeline
  (`TimelineComponent.SetPlayRate` (`self.CrosairTimeline`) 5.0))

(event `Crosshair`
  (bind _firstpersoncamera (`self.FirstPersonCamera`))
  (bind _returnvalue (`SceneComponent.K2_GetComponentLocation` _firstpersoncamera))
  ;[0 0 0] Crosshair Animation Material
  ;;[1 1 1] Gizmo vom Crosshair
  (bind (_outhit _returnvalue_2) (`KismetSystemLibrary.LineTraceSingle` :`Start` _returnvalue :`End` (+ _returnvalue (* (`KismetMathLibrary.Normal` (`SceneComponent.GetForwardVector` _firstpersoncamera)) 150.0)) :`TraceChannel` "TraceTypeQuery1" :`TraceColor` (struct :`R` 0.322784 :`G` 0.309979 :`B` 1.0 :`A` 1.0) :`DrawTime` 1.0)) ; Setzt und Start und Ende des geschossenen Punkts
  ;;[1 1 1] Abfrage vom Interactable
  (if _returnvalue_2
    (bind (_bblockinghit _binitialoverlap _time _distance _location _impactpoint _normal _impactnormal _physmat _hitactor) (`GameplayStatics.BreakHitResult` _outhit))
    (bind _isinteractable (message `/Game/01_DEV/Interactables/Interface_Interactable.Valid` _hitactor))
    (if _isinteractable
      ;;[1 1 1] Füllt/Leert
      (set `self.CurrentInteractable` _hitactor)
      ;;[1 1 1] Lerp vom Material
      ;;;[0.1119 0.4969 0.5906] TimeLine
      (bind (_direction _value) (`Timeline|CrosairTimeline` :!label _label)
        (:`Update`
          (`KismetMaterialLibrary.SetScalarParameterValue` "/Game/02_UI/Crosshair/MPC_Crosshair.MPC_Crosshair" "CanInteract" _value) ; Material Gruppe
        ))
      (else
        (set `self.CurrentInteractable` null :!label _label_2)
        (goto _label :!via `Reverse`)))
    (else
      (goto _label_2))))

(event `CurrentInventory`
  (params (SetItem :type Boolean))
  (bind _returnvalue (`KismetArrayLibrary.Array_Add` (`self.Inventory`) SetItem))
  (set `self.CurrentIntemIndex` _returnvalue)
  (`self.ShowItem`))

(event `ShowItem`
  (bind _itemmesh (`self.ItemMesh`))
  (if true
    (`SceneComponent.SetVisibility` (`self.ItemMesh`) false false)
    (else
      (`SceneComponent.SetVisibility` (`self.ItemMesh`) true false)
      (`StaticMeshComponent.SetStaticMesh` _itemmesh null)
      (for (_array_element _array_index) _
        (`PrimitiveComponent.SetMaterial` _itemmesh _array_index _array_element)))))

(event `EnhancedInput|/Game/01_DEV/Input/IA_Interact`
  (params (ActionValue :type Boolean) (ElapsedSeconds :type "Float (double-precision)") (TriggeredSeconds :type "Float (double-precision)") (InputAction :type "InputAction Object Reference" :default "/Game/01_DEV/Input/IA_Interact.IA_Interact"))
  ;[1 0.7744 0.1821] Interactable
  (:`Started`
    (if (`self.CanMove`)
      (bind _currentinteractable (`self.CurrentInteractable`)
        (:`then`
          (message `/Game/01_DEV/Interactables/Interface_Interactable.Interact` _currentinteractable self))
        (:`else`)))))

(event `EnhancedInput|/Game/01_DEV/Input/IA_Look`
  (params (ActionValue :type "Vector2D Structure") (ElapsedSeconds :type "Float (double-precision)") (TriggeredSeconds :type "Float (double-precision)") (InputAction :type "InputAction Object Reference" :default "/Game/01_DEV/Input/IA_Look.IA_Look"))
  ;[0.2623 0.5906 1] Look
  (:`Triggered`
    (if (`self.CanMove`)
      (`self.AddControllerYawInput` ActionValue_X)
      (`self.AddControllerPitchInput` ActionValue_Y))))

(event `EnhancedInput|/Game/01_DEV/Input/IA_Move`
  (params (ActionValue :type "Vector2D Structure") (ElapsedSeconds :type "Float (double-precision)") (TriggeredSeconds :type "Float (double-precision)") (InputAction :type "InputAction Object Reference" :default "/Game/01_DEV/Input/IA_Move.IA_Move"))
  ;[0.2623 0.5906 1] Move
  (:`Triggered`
    (if (`self.CanMove`)
      (`self.AddMovementInput` (`self.GetActorRightVector`) ActionValue_X)
      (`self.AddMovementInput` (`self.GetActorForwardVector`) ActionValue_Y))))

(fn `UserConstructionScript`)