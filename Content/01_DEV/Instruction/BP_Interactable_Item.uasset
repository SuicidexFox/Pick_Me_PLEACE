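; BP_Interactable_Item is an interactable item Blueprint with a static mesh, apparently intended for player pickup into an inventory.
; Its Interact event is currently empty, and disconnected nodes reference the player's current inventory and the mesh's transform, class and material.
; Valid reports it as not interactable with the first type enum value, and SetSolved always returns false, so it functions as a stub.
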(event `/Game/01_DEV/Interactables/Interface_Interactable.Interact`
  (params (Player_ID :type "/Game/01_DEV/BP_Player Object Reference")))

(fn `SetSolved`
  (returns (SetSolved :type Boolean))
  (return false))

(fn `UserConstructionScript`)

(fn `Valid`
  (returns (Interactable :type Boolean) (Typ :type "/Game/01_DEV/Interactables/E_Interactable_Type Enum"))
  (return false "NewEnumerator0"))