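; Inspectable interactable pawn that brings its object in front of the player's view for examination and rotation.
; Interact snaps its camera to the player's, takes possession, eases the Scene component forward, hides the held item and adds an inspect widget.
; Move input rotates the object on one axis.
; Interact input eases it back, restores possession and control rotation; the widget-removal call is never reached.
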(event `self.ReceiveBeginPlay`
  (set `self.StartTransform` (`SceneComponent.GetRelativeTransform` (`self.Scene`))))

(event `/Game/01_DEV/Interactables/Interface_Interactable.Interact`
  (params (Player_ID :type "/Game/01_DEV/BP_Player_0 Object Reference"))
  (bind _returnvalue (`GameplayStatics.GetPlayerController` 0))
  (bind _camera (`self.Camera`))
  (bind (_returnvalue_location _returnvalue_rotation) (`KismetMathLibrary.BreakTransform` (`SceneComponent.GetRelativeTransform` _camera)))
  ;[1 1 1] Interact
  (bind _output_get (set `self.Player ID` Player_ID))
  (bind (_returnvalue_location_2 _returnvalue_rotation_2) (`KismetMathLibrary.BreakTransform` (`SceneComponent.K2_GetComponentToWorld` (`/Game/01_DEV/BP_Player_0.FirstPersonCamera` _output_get))))
  ;;[1 0.4852 0.05286] Cam Bewegt sich zu unserer Cam
  (`SceneComponent.K2_SetWorldLocationAndRotation` (`self.Camera`) _returnvalue_location_2 _returnvalue_rotation_2 false true)
  (set `self.PlayerControllerRotation` (`Controller.GetControlRotation` _returnvalue))
  (`Controller.Possess` _returnvalue self) ; Inputs werden\nPawn übergeben
  (`|ExecutionSequence`
    (:`then_1`
      ;;[1 0.4852 0.05286] Scene bewegt sich vor unsere Camera
      (`KismetSystemLibrary.MoveComponentTo` (`self.Scene`) (+ _returnvalue_location (* (`KismetMathLibrary.Normal` (`SceneComponent.GetForwardVector` _camera)) (`self.Distance`))) _returnvalue_rotation true true 1.0)
      (set `self.IsInspacted` true)
      (`self.ToggleUIInspact`))))

(event `ToggleUIInspact`
  (bind _itemmesh (`/Game/01_DEV/BP_Player_0.ItemMesh` (`self.Player ID`)))
  ;[1 1 1] UI wird aufgerufen
  (`/Engine/EditorBlueprintResources/StandardMacros.FlipFlop`
    (:`A`
      (`SceneComponent.SetVisibility` _itemmesh false false)
      (bind _returnvalue (`CommonActivatableWidgetContainerBase.BP_AddWidget` (`/Game/01_DEV/FL_Utils.Set Up Widget Stack` (`GameplayStatics.GetPlayerController` 0)) "/Game/02_UI/ABW_Inspacted.ABW_Inspacted_C"))
      (set `self.CurrentWidget` _returnvalue))
    (:`B`
      (`SceneComponent.SetVisibility` _itemmesh true false))))

(event `EnhancedInput|/Game/01_DEV/Input/IA_Interact`
  (params (ActionValue :type Boolean) (ElapsedSeconds :type "Float (double-precision)") (TriggeredSeconds :type "Float (double-precision)") (InputAction :type "InputAction Object Reference" :default "/Game/01_DEV/Input/IA_Interact.IA_Interact"))
  (bind _returnvalue (`GameplayStatics.GetPlayerController` 0))
  (bind (_starttransform_location _starttransform_rotation) (`KismetMathLibrary.BreakTransform` (`self.StartTransform`)))
  ;[1 1 1] Leave
  (:`Started`
    (if (`self.IsInspacted`)
      (set `self.IsInspacted` false)
      ;;[1 0.4852 0.05286] Scene move to Start
      (`KismetSystemLibrary.MoveComponentTo` (`self.Scene`) _starttransform_location _starttransform_rotation true true 1.0)
      (`Controller.Possess` _returnvalue (`self.Player ID`)) ; Inputs werden\nan Player übergeben
      (`Controller.SetControlRotation` _returnvalue (`self.PlayerControllerRotation`))
      (`self.ToggleUIInspact`))))

(event `EnhancedInput|/Game/01_DEV/Input/IA_Move`
  (params (ActionValue :type "Vector2D Structure") (ElapsedSeconds :type "Float (double-precision)") (TriggeredSeconds :type "Float (double-precision)") (InputAction :type "InputAction Object Reference" :default "/Game/01_DEV/Input/IA_Move.IA_Move"))
  (bind (_returnvalue_roll _returnvalue_pitch) (`KismetMathLibrary.BreakRotator` (`KismetMathLibrary.MakeRotator` 0.0 (* ActionValue_Y -4.0))))
  (:`Triggered`
    (`SceneComponent.K2_AddLocalRotation` (`self.Scene`) (`KismetMathLibrary.MakeRotator` _returnvalue_pitch) false true)))

(fn `SetSolved`
  (returns (IsSolved :type Boolean))
  (return false))

(fn `Targeted`
  (return))

(fn `Untargeted`
  (return))

(fn `UserConstructionScript`)

(fn `Valid`
  (returns (IsInteractable :type Boolean) (Typ :type "/Game/01_DEV/Interactables/E_Interactable_Type Enum"))
  (return (`self.IsInteractable`) "NewEnumerator0"))