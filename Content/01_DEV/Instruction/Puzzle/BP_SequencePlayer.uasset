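; BP_SequencePlayer is a non-interactable puzzle actor that plays a level sequence once when solved.
; During playback it disables player movement and clears the crosshair stack, restoring both when the sequence finishes.
; In parallel, after a configurable delay, it sends a solved message to its linked actors, and forwards unsolved messages immediately.
; Repeat solves skip playback but still lock the player and rebind the finish callback.
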(event `/Game/01_DEV/Interactables/Interface_Interactable.Solved`
  (`|ExecutionSequence`
    (:`then_0`
      (bind _sequence (`self.Sequence`)
        (:`then`
          (`/Engine/EditorBlueprintResources/StandardMacros.DoOnceWithAfter`
            (:`Once`
              (`MovieSceneSequencePlayer.Play` (`LevelSequenceActor.SequencePlayer` _sequence))
              (bind _asbp_player (cast `/Game/01_DEV/BP_Player` (`GameplayStatics.GetPlayerCharacter` 0)))
              (set `self.BP Player` _asbp_player))
            (:`After`
              _))
          (set `/Game/01_DEV/BP_Player.CanMove` false (`self.BP Player`))
          (`CommonActivatableWidgetContainerBase.ClearWidgets` (`/Game/01_DEV/FL_Utils.Set Up Widget Stack` (`GameplayStatics.GetPlayerController` 0)))
          (add `MovieSceneSequencePlayer.OnFinished` (`LevelSequenceActor.SequencePlayer` (`self.Sequence`)) (delegate `SenceEnd`)))
        (:`else`)))
    (:`then_1`
      (`KismetSystemLibrary.Delay` (`self.DurationStartSequence`))
      (for _array_element (`self.ActorToReact`)
        (message `/Game/01_DEV/Interactables/Interface_Interactable.Solved` _array_element)))))

(event `SenceEnd`
  (set `/Game/01_DEV/BP_Player.CanMove` true (`self.BP Player`))
  (`CommonActivatableWidgetContainerBase.BP_AddWidget` (`/Game/01_DEV/FL_Utils.Set Up Widget Stack` (`GameplayStatics.GetPlayerController` 0)) "/Game/02_UI/Crosshair/AWB_Crosshair.AWB_Crosshair_C"))

(event `/Game/01_DEV/Interactables/Interface_Interactable.Unsolved`
  (for _array_element (`self.ActorToReact`)
    (message `/Game/01_DEV/Interactables/Interface_Interactable.Unsolved` _array_element)))

(fn `SetSolved`
  (returns (SetSolved :type Boolean))
  (return false))

(fn `UserConstructionScript`)

(fn `Valid`
  (returns (Interactable :type Boolean) (Typ :type "/Game/01_DEV/Interactables/E_Interactable_Type Enum"))
  (return false "NewEnumerator4"))