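; BP_SequencePlayer is a non-interactable actor that relays solved and unsolved messages to the objects in its TimeLater array.
; Solved forwards SolvedMessage after a one-second delay, while Unsolved forwards UnsolvedMessage immediately.
; Despite the name, Solved only validity-checks the Sequence without playing it.
; The logic to play it, lock player movement and hide the crosshair until it ends is disconnected and never runs.
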(event `/Game/01_DEV/Interactables/Interface_Interactable.Solved`
  (`|ExecutionSequence`
    (:`then_0`
      (bind _sequence (`self.Sequence`)
        (:`then`)
        (:`else`)))
    (:`then_1`
      (`KismetSystemLibrary.Delay` 1.0)
      (for _array_element (`self.TimeLater`)
        (message `/Game/01_DEV/Interactables/Interface_Interactable.Solved` _array_element)))))

(event `/Game/01_DEV/Interactables/Interface_Interactable.Unsolved`
  (for _array_element (`self.TimeLater`)
    (message `/Game/01_DEV/Interactables/Interface_Interactable.Unsolved` _array_element)))

(fn `SetSolved`
  (returns (IsSolved :type Boolean))
  (return false))

(fn `UserConstructionScript`)

(fn `Valid`
  (returns (IsInteractable :type Boolean) (Typ :type "/Game/01_DEV/Interactables/E_Interactable_Type Enum"))
  (return false "NewEnumerator4"))