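; BP_ItemSocket is an interactable socket where a player places the selected inventory item, acting as a puzzle condition when it needs a specific item.
; Interact spawns any held item at the socket, links it back via CurrentSocket and removes it from the inventory.
; A name matching NeedItem marks the socket solved and messages ActorsToReact.
; It reports interactable only while enabled and empty, and SetValid forwards that enabled state to the placed item.
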(event `/Game/01_DEV/Interface_and_Self/Interface_Interactable.Interact`
  (params (Player_ID :type "/Game/01_DEV/BP_Player Object Reference"))
  (bind _inventory (`/Game/01_DEV/BP_Player.Inventory` Player_ID))
  (bind _currentintemindex (`/Game/01_DEV/BP_Player.CurrentIntemIndex` Player_ID))
  (bind (_scene _name _mesh _materials _transform _class) (break `/Game/01_DEV/Interactables/ItemStructure` (`|GetArrayItem` _inventory _currentintemindex)))
  (if (`KismetStringLibrary.NotEqual_StrStr` _name)
    (`self.CurrentItem`
      (:`then`)
      (:`else`
        (bind _returnvalue (`|SpawnActorFromClass` _class (`SceneComponent.K2_GetComponentToWorld` (`self.Scene`)) "Undefined" "MultiplyWithRoot" null null))
        (bind _output_get (set `self.CurrentItem` _returnvalue))
        (bind _asbp_interactable_item (cast `/Game/01_DEV/Instruction/BP_Interactable_Item` _output_get))
        (set `/Game/01_DEV/Instruction/BP_Interactable_Item.CurrentSocket` self _asbp_interactable_item)
        (if (`KismetStringLibrary.EqualEqual_StrStr` (`.Name_5_1C06FF694E268D40E70FD589ADD5300D` (break `/Game/01_DEV/Interactables/ItemStructure` (`|GetArrayItem` _inventory _currentintemindex))) (`self.NeedItem`))
          (set `self.Set Solved` true)
          (for _array_element (`self.ActorsToReact`)
            (message `/Game/01_DEV/Interface_and_Self/Interface_Interactable.Solved` _array_element)))
        (`KismetArrayLibrary.Array_Remove` _inventory _currentintemindex)
        (`/Engine/EditorBlueprintResources/StandardMacros.DecrementInt` _currentintemindex
          (:`  `
            (`/Game/01_DEV/BP_Player.ShowItem` Player_ID)))))))

(event `/Game/01_DEV/Interface_and_Self/Interface_Interactable.SetValid`
  (params (SetValid :type Boolean))
  (bind _output_get (set `self.SetInteractable` SetValid))
  (message `/Game/01_DEV/Interface_and_Self/Interface_Interactable.SetValid` (`self.CurrentItem`) _output_get))

(fn `SetSolved`
  (returns (SetSolved :type Boolean))
  (return (`self.Set Solved`)))

(fn `UserConstructionScript`)

(fn `Valid`
  (returns (Interactable :type Boolean) (Typ :type "/Game/01_DEV/Interactables/E_Interactable_Type Enum"))
  (return (and (`self.SetInteractable`) (not (`KismetSystemLibrary.IsValid` (`self.CurrentItem`)))) "NewEnumerator6"))