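; Interactable object that moves and rotates its Scene component to a target transform when used, either once or as a back-and-forth toggle.
; Interact runs an eased MoveComponentTo behind a DoOnce gate, blocking retriggers mid-move.
; On completion, the DoOnce variable either disables interaction or lets a FlipFlop swap start and target and reset the gate.
; Solved and Unsolved are empty, and SetSolved always returns false.
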(event `self.ReceiveBeginPlay`
  (set `self.StartTransform` (`SceneComponent.GetRelativeTransform` (`self.Scene`)))
  (set `self.CurrentTransform` (`self.TargetTransform`)))

(event `/Game/01_DEV/Interactables/Interface_Interactable.Solved`)

(event `/Game/01_DEV/Interactables/Interface_Interactable.Unsolved`)

(event `/Game/01_DEV/Interactables/Interface_Interactable.Interact`
  (params (Player_ID :type "/Game/01_DEV/BP_Player Object Reference"))
  (`/Engine/EditorBlueprintResources/StandardMacros.DoOnce` false :!label _label ; feuert ein Mal
    (:`Completed`
      (`KismetSystemLibrary.MoveComponentTo` (`self.Scene`) (.location (`self.CurrentTransform`)) (.rotation (`self.CurrentTransform`)) true true (`self.MoveDuration`) true)
      (if (`self.DoOnce`)
        (set `self.IsInteractable` false)
        (else
          (`/Engine/EditorBlueprintResources/StandardMacros.FlipFlop`
            (:`A`
              (set `self.CurrentTransform` (`self.StartTransform`)))
            (:`B`
              (set `self.CurrentTransform` (`self.TargetTransform`))))
          (`|ExecutionSequence`
            (:`then_1`
              (goto _label :!via `Reset`))))))))

(fn `SetSolved`
  (returns (IsSolved :type Boolean))
  (return false))

(fn `UserConstructionScript`)

(fn `Valid`
  (returns (IsInteractable :type Boolean) (Typ :type "/Game/01_DEV/Interactables/E_Interactable_Type Enum"))
  (return (`self.IsInteractable`) (`self.Typ`)))