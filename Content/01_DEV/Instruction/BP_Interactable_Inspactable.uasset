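; Interactable actor for inspecting an object: interacting slides it from its start transform along the player camera's forward vector by a set Distance, using a Timeline.
; Move input pitches the mesh, and interface functions report interactability and type, with the others left as stubs.
; An Interact-input exit restores possession, control rotation and mesh position, but its IsInspacted flag is only set in disconnected code, alongside older possession, camera and widget logic.
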(event `self.ReceiveBeginPlay`
  (set `self.StartTransform` (`self.GetTransform`)))

(event `/Game/01_DEV/Interactables/Interface_Interactable.Interact`
  (params (Player_ID :type "/Game/01_DEV/BP_Player Object Reference"))
  (bind _starttransform_location (`KismetMathLibrary.BreakTransform` (`self.StartTransform`)))
  (bind _output_get (set `self.PlayerID` Player_ID))
  (bind (_direction _newtrack_0) (`Timeline|Timeline` :!via `PlayFromStart`)
    (:`Update`
      (bind _firstpersoncamera (`/Game/01_DEV/BP_Player.FirstPersonCamera` _output_get))
      (bind _returnvalue_location (`KismetMathLibrary.BreakTransform` (`KismetMathLibrary.TLerp` (`self.StartTransform`) (`KismetMathLibrary.MakeTransform` (+ _starttransform_location (* (`KismetMathLibrary.Normal` (`SceneComponent.GetForwardVector` _firstpersoncamera)) (`self.Distance`))) (`SceneComponent.K2_GetComponentRotation` _firstpersoncamera)) _newtrack_0)))
      (`self.K2_SetActorLocationAndRotation` _returnvalue_location))))

(event `EnhancedInput|/Game/01_DEV/Input/IA_Move`
  (params (ActionValue :type "Vector2D Structure") (ElapsedSeconds :type "Float (double-precision)") (TriggeredSeconds :type "Float (double-precision)") (InputAction :type "InputAction Object Reference" :default "/Game/01_DEV/Input/IA_Move.IA_Move"))
  (bind (_returnvalue_roll _returnvalue_pitch) (`KismetMathLibrary.BreakRotator` (`KismetMathLibrary.MakeRotator` 0.0 (* ActionValue_Y -4.0))))
  (:`Triggered`
    (`SceneComponent.K2_AddLocalRotation` (`self.Mesh`) (`KismetMathLibrary.MakeRotator` _returnvalue_pitch) false true)))

(event `EnhancedInput|/Game/01_DEV/Input/IA_Interact`
  (params (ActionValue :type Boolean) (ElapsedSeconds :type "Float (double-precision)") (TriggeredSeconds :type "Float (double-precision)") (InputAction :type "InputAction Object Reference" :default "/Game/01_DEV/Input/IA_Interact.IA_Interact"))
  (bind _returnvalue (`GameplayStatics.GetPlayerController` 0))
  (bind (_starttransform_location _starttransform_rotation) (`KismetMathLibrary.BreakTransform` (`self.StartTransform`)))
  ;[1 1 1] Leave
  (:`Started`
    (if (`self.IsInspacted`)
      (set `self.IsInspacted` false)
      (`|ExecutionSequence`
        (:`then_0`
          (`Controller.Possess` _returnvalue (`self.PlayerID`)) ; Inputs werden\nan Player übergeben
          ;;[1 0.4852 0.05286] Scene move to Start
          (`KismetSystemLibrary.MoveComponentTo` (`self.Mesh`) _starttransform_location _starttransform_rotation true true 1.0 true)
          (set `/Game/01_DEV/BP_Player.CanMove` true (`self.PlayerID`)))
        (:`then_1`
          (`Controller.SetControlRotation` _returnvalue (`self.PlayerControllerRotation`))
          (`KismetSystemLibrary.MoveComponentTo` null (-105.0 0.0 0.0) (struct) true true 1.0 true))))))

(fn `SetSolved`
  (returns (IsSolved :type Boolean))
  (return false))

(fn `Targeted`
  (return))

(fn `Untargeted`
  (return))

(fn `UserConstructionScript`)

(fn `Valid`
  (returns (IsInteractable :type Boolean) (Typ :type "/Game/01_DEV/Interactables/E_Interactable_Type Enum"))
  (return (`self.IsInteractable`) (`self.Type`)))