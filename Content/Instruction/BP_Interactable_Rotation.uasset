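; Interactable puzzle piece that rotates its mesh through a looping list of preset rotations, one eased step per interaction.
; A DoOnce gate blocks re-entry until the move and solve check finish.
; Reaching the correct position sends a solved message to linked actors and optionally disables interaction; leaving it sends an unsolved message.
; The construction script applies only the starting position's pitch to the mesh.
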(event `/Game/01_DEV/Interface_and_Self/Interface_Interactable.Interact`
  (params (Player_ID :type "/Game/01_DEV/BP_Player Object Reference"))
  (bind _currentposition (`self.CurrentPosition`))
  (bind _rotationpositions (`self.RotationPositions`))
  (bind _mesh (`self.Mesh`))
  (bind _returnvalue (+ _currentposition 1))
  (`/Engine/EditorBlueprintResources/StandardMacros.DoOnce` false :!label _label
    (:`Completed`
      (set `self.CurrentPosition` (`KismetMathLibrary.SelectInt` 0 _returnvalue (> _returnvalue (`KismetArrayLibrary.Array_LastIndex` _rotationpositions))))
      (`KismetSystemLibrary.MoveComponentTo` _mesh (`SceneComponent.RelativeLocation` _mesh) (`|GetArrayItem` _rotationpositions _currentposition) true true 0.5)
      (if (== (`self.CurrentPosition`) (`self.CorrectPosition`))
        (set `self.Current Solved` true)
        (if (`self.StopPuzzle`)
          (`|ExecutionSequence`
            (:`then_0`
              _)
            (:`then_1`
              (set `self.Set Interactable` false)
              (for _array_element (`self.ActorToReact`) :!label _label_2
                (message `/Game/01_DEV/Interface_and_Self/Interface_Interactable.Solved` _array_element))
              (goto _label :!via `Reset`)))
          (else
            (`|ExecutionSequence`
              (:`then_0`
                _)
              (:`then_1`
                (goto _label_2)))))
        (`/Engine/EditorBlueprintResources/StandardMacros.DoOnce` false)
        (elif (`self.Current Solved`)
          (set `self.Current Solved` false)
          (for _array_element_2 (`self.ActorToReact`)
            (message `/Game/01_DEV/Interface_and_Self/Interface_Interactable.Unsolved` _array_element_2))
          (goto _label :!via `Reset`)
          (else
            (goto _label :!via `Reset`)))))))

(event `/Game/01_DEV/Interface_and_Self/Interface_Interactable.SetValid`
  (params (SetValid :type Boolean))
  (set `self.Set Interactable` SetValid))

(fn `SetSolved`
  (returns (SetSolved :type Boolean))
  (return (`self.Set Interactable`)))

(fn `UserConstructionScript`
  (bind (_output_roll _output_pitch) (`KismetMathLibrary.BreakRotator` (`|GetArrayItem` (`self.RotationPositions`) (`self.CurrentPosition`))))
  (`SceneComponent.K2_SetRelativeRotation` (`self.Mesh`) (`KismetMathLibrary.MakeRotator` 0.0 _output_pitch) false true))

(fn `Valid`
  (returns (Interactable :type Boolean) (Typ :type "/Game/01_DEV/Puzzle/E_Interactable_Type Enum"))
  (return (`self.Set Interactable`) "NewEnumerator3"))