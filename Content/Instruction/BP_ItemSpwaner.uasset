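; BP_ItemSpwaner is an actor that spawns a collectable of a configurable class at its own transform when its Solved event fires.
; It tracks the spawned actor and only spawns again once that actor is no longer valid.
; An Only flag routes through a DoOnce meant to limit spawning.
; Its Solved and Valid functions report it as unsolved and non-interactable.
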(event `Solved_1_1`
  (`self.CurrentActor`
    (:`then`)
    (:`else`
      (if (`self.Only`)
        (`/Engine/EditorBlueprintResources/StandardMacros.DoOnce` false
          (:`Completed`
            _)))
      (bind _returnvalue (`|SpawnActorFromClass` (`self.Collectable Class`) (`self.GetTransform`) "Undefined" "MultiplyWithRoot" null null))
      (set `self.CurrentActor` _returnvalue))))

(fn `Solved`
  (returns (SetSolved :type Boolean))
  (return false))

(fn `UserConstructionScript`)

(fn `Valid`
  (returns (Interactable :type Boolean) (Typ :type "/Game/01_DEV/Puzzle/E_Interactable_Type Enum"))
  (return false "NewEnumerator0"))