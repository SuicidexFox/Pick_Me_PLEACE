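; BP_SequencePlayer is a non-interactable puzzle-chain actor that plays a level sequence when solved and relays solved or unsolved messages to linked actors.
; The sequence plays only the first time, but every trigger with a valid sequence disables player movement and clears the HUD.
; The sequence's finish event restores both.
; Linked actors get the solved message after a configurable delay, while unsolved messages pass through immediately.
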(event `Solved_1_1`
  (`|ExecutionSequence`
    (:`then_0`
      (bind _sequence (`self.Sequence`)
        (:`then`
          (`/Engine/EditorBlueprintResources/StandardMacros.DoOnceWithAfter`
            (:`Once`
              (`MovieSceneSequencePlayer.Play` (`LevelSequenceActor.SequencePlayer` _sequence))
              (bind _asbp_player (cast `/Game/01_DEV/BP_Player` (`GameplayStatics.GetPlayerCharacter` 0)))
              (set `self.BP Player` _asbp_player))
            (:`After`
              _))
          (set `/Game/01_DEV/BP_Player.CanMove` false (`self.BP Player`))
          (`CommonActivatableWidgetContainerBase.ClearWidgets` (`/Game/01_DEV/Interface_and_Self/FL_Utils.GetOverlayStacks` (`GameplayStatics.GetPlayerController` 0)))
          (add `MovieSceneSequencePlayer.OnFinished` (`LevelSequenceActor.SequencePlayer` (`self.Sequence`)) (delegate `SenceEnd`)))
        (:`else`)))
    (:`then_1`
      (`KismetSystemLibrary.Delay` (`self.DurationStartSequence`))
      (for _array_element (`self.ActorToReact`)
        (message `/Game/01_DEV/Interface_and_Self/Interface_Interactable.Solved` _array_element)))))

(event `SenceEnd`
  (set `/Game/01_DEV/BP_Player.CanMove` true (`self.BP Player`))
  (`CommonActivatableWidgetContainerBase.BP_AddWidget` (`/Game/01_DEV/Interface_and_Self/FL_Utils.GetOverlayStacks` (`GameplayStatics.GetPlayerController` 0)) "/Game/03_UI/AWB_PlayerHUD.AWB_PlayerHUD_C"))

(event `/Game/01_DEV/Interface_and_Self/Interface_Interactable.SetUnsolved`
  (for _array_element (`self.ActorToReact`)
    (message `/Game/01_DEV/Interface_and_Self/Interface_Interactable.SetUnsolved` _array_element)))

(fn `Solved`
  (returns (SetSolved :type Boolean))
  (return false))

(fn `UserConstructionScript`)

(fn `Valid`
  (returns (Interactable :type Boolean) (Typ :type "/Game/01_DEV/Puzzle/E_Interactable_Type Enum"))
  (return false "NewEnumerator4"))