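; BP_Lookpick is an unfinished interactable, apparently a lockpick minigame pawn, that reports itself non-interactable and unsolved.
; Interact stores the player, saves control rotation and disables movement, but the possess, widget and fade-in steps are disconnected.
; The interact input reverses a timeline driving material opacity and scene transform, then repossesses the player with the saved rotation.
; Move and Space inputs route to empty directional handlers behind an IsNotMoving gate that is never reset.
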(event `self.ReceiveBeginPlay`
  (bind _mash (`self.Mash`))
  (bind _returnvalue (`PrimitiveComponent.CreateDynamicMaterialInstance` _mash 0 (`PrimitiveComponent.GetMaterial` _mash 0) "None"))
  (set `self.Material` _returnvalue))

(event `/Game/01_DEV/Interface_and_Self/Interface_Interactable.SetValid`
  (params (SetValid :type Boolean))
  (set `self.IsInteracted` SetValid))

(event `/Game/01_DEV/Interface_and_Self/Interface_Interactable.Interact`
  (params (Player_ID :type "/Game/01_DEV/BP_Player Object Reference"))
  (bind _playerid (`self.PlayerID`))
  (set `self.PlayerID` Player_ID)
  (set `self.ControlRotation` (`self.GetControlRotation` _playerid))
  (set `/Game/01_DEV/BP_Player.CanMove` false _playerid))

(event `EnhancedInput|/Game/01_DEV/Input/IA_Interact`
  (params (ActionValue :type Boolean) (ElapsedSeconds :type "Float (double-precision)") (TriggeredSeconds :type "Float (double-precision)") (InputAction :type "InputAction Object Reference" :default "/Game/01_DEV/Input/IA_Interact.IA_Interact"))
  (bind _returnvalue (`GameplayStatics.GetPlayerController` 0))
  (:`Started`
    (`self.SetupMaterial` false)
    (`Controller.Possess` _returnvalue (`self.PlayerID`)) ; shmoot possess
    (`Controller.SetControlRotation` _returnvalue (`self.ControlRotation`))))

(event `SetupMaterial`
  (params (FadeOut :type Boolean))
  (if FadeOut
    (bind (_direction _value) (`Timeline|FadeTimeline` :!label _label)
      (:`Update`
        (`MaterialInstanceDynamic.SetScalarParameterValue` (`self.Material`) "Opacity" (`KismetMathLibrary.Lerp` 0.1 1.0 _value))
        (`SceneComponent.K2_SetRelativeTransform` (`self.Scene`) (`KismetMathLibrary.MakeTransform` (0.0 0.0 0.0) (`KismetMathLibrary.RLerp` (struct :`Yaw` 90.0) (struct) _value) (`KismetMathLibrary.Vector_SlerpNormals` (1.0 0.2 1.0) (1.0 1.0 1.0) _value)) true false)))
    (else
      (goto _label :!via `Reverse`))))

(event `EnhancedInput|/Game/01_DEV/Input/IA_Move`
  (params (ActionValue :type "Vector2D Structure") (ElapsedSeconds :type "Float (double-precision)") (TriggeredSeconds :type "Float (double-precision)") (InputAction :type "InputAction Object Reference" :default "/Game/01_DEV/Input/IA_Move.IA_Move"))
  (:`Started`
    (if (`self.IsNotMoving`)
      (set `self.IsNotMoving` false)
      (if (> (`KismetMathLibrary.Abs` ActionValue_X) (`KismetMathLibrary.Abs` ActionValue_Y))
        (`self.Left/Right` ActionValue_X)
        (else
          (`self.Up/Down` ActionValue_Y))))))

(event `EnhancedInput|/Game/01_DEV/Input/IA_Space`
  (params (ActionValue :type Boolean) (ElapsedSeconds :type "Float (double-precision)") (TriggeredSeconds :type "Float (double-precision)") (InputAction :type "InputAction Object Reference" :default "/Game/01_DEV/Input/IA_Space.IA_Space"))
  (:`Started`
    (if (`self.IsNotMoving`)
      (set `self.IsNotMoving` false)
      (`self.Up/Down` 1.0))))

(event `Left/Right`
  (params (x :type "Float (double-precision)"))
  (if (> x 0.0)
    _))

(event `Up/Down`
  (params (y :type "Float (double-precision)"))
  (if (> y 0.0)
    _))

(fn `SetSolved`
  (returns (SetSolved :type Boolean))
  (return false))

(fn `UserConstructionScript`)

(fn `Valid`
  (returns (Interactable :type Boolean) (Typ :type "/Game/01_DEV/Puzzle/E_Interactable_Type Enum"))
  (return false "NewEnumerator4"))