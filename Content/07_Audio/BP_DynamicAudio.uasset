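; BP_DynamicAudio is an audio actor that builds up the music as Solved events arrive.
; BeginPlay spawns MS_Music as a 2D sound and keeps a reference to it.
; While Gain is below a cap, Solved plays a timeline that ramps the OverallGain parameter up from the current Gain, then increments Gain.
; SetSolved and Valid return fixed values, marking the actor as non-interactable.
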(event `self.ReceiveBeginPlay`
  (bind _returnvalue (`GameplayStatics.SpawnSound2D` "/Game/07_Audio/MS_Music.MS_Music" 1.0 1.0 0.0 null))
  (set `self.MusicAmbience` _returnvalue))

(event `/Game/01_DEV/Interface_and_Self/Interface_Interactable.Solved`
  (if (< (`self.Gain`) 2.0)
    (bind (_direction _value) (`Timeline|GainTimeline` :!via `PlayFromStart`)
      (:`Update`
        (`AudioComponent.SetFloatParameter` (`self.MusicAmbience`) "OverallGain" (+ _value (`self.Gain`))))
      (:`Finished`
        (bind _result (`/Engine/EditorBlueprintResources/StandardMacros.IncrementFloat` (`self.Gain`))
          (:`  `
            (`AudioComponent.SetFloatParameter` (`self.MusicAmbience`) "OverallGain" _result)))))))

(fn `SetSolved`
  (returns (SetSolved :type Boolean))
  (return false))

(fn `UserConstructionScript`)

(fn `Valid`
  (returns (Interactable :type Boolean) (Typ :type "/Game/01_DEV/Puzzle/E_Interactable_Type Enum"))
  (return false "NewEnumerator4"))